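; Pistol weapon Blueprint that adds firing effects and magazine handling on top of its parent class.
; SpecialFx restarts the muzzle particle and plays a timeline that slides two pistol meshes, the second through a remapped offset.
; Unload hides the magazine and, on authority, spawns an ammo actor carrying the current count; Reload restores the magazine, and both trigger weapon noise.
; Construction takes Ammo from the ammo class defaults when loaded, otherwise hides the magazine.
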(event `self.SpecialFx`
  (`|ExecutionSequence`
    (:`then_0`
      ;[1 1 1] Fire Particle
      (`ActorComponent.SetActive` (`self.FireGun`) true true))
    (:`then_1`
      ;[1 1 1] MoveSecondPart
      (bind (_direction _gunpartmove) (`Timeline|PistolPartMove` :!via `PlayFromStart`)
        (:`Update`
          (`SceneComponent.K2_SetRelativeLocation` (`self.StaticMesh`) (`KismetMathLibrary.MakeVector` 0.0 _gunpartmove) false false)
          (`SceneComponent.K2_SetRelativeLocation` (`self.StaticMesh1`) (`KismetMathLibrary.MakeVector` 0.0 (`KismetMathLibrary.MapRangeClamped` _gunpartmove 0.0 -3.0 0.0 2.0)) false false))))))

(event `self.Unload`
  ;[1 1 1] UnloadWeapon
  (if (`self.Loaded`)
    (`self.ArmeBruit` true)
    (`KismetSystemLibrary.MoveComponentTo` (`self.Cartouche`) (0.0 3.0 -8.0))
    (`SceneComponent.SetVisibility` (`self.Cartouche`) false false)
    (`/Engine/EditorBlueprintResources/ActorMacros.Switch Has Authority`
      (:`Authority`
        (set `self.Loaded` false)
        (bind _returnvalue (`|SpawnActorFromClass` (`self.AmmoType`) (`SceneComponent.K2_GetComponentToWorld` (`self.Cartouche`)) "AlwaysSpawn" "OverrideRootScale" null null))
        (set `/Game/JustATestAssets/Environnement/Usable/Items/Weapon/Ammo/AmmoBP.Ammo` (`self.Ammo`) _returnvalue)))))

(event `self.Reload`
  (bind _cartouche (`self.Cartouche`))
  ;[1 1 1] ReloadWeapon
  (`SceneComponent.SetVisibility` _cartouche true false)
  (set `self.Loaded` true)
  (`SceneComponent.K2_SetRelativeLocation` _cartouche (0.0 0.0 0.0) false false)
  (`self.ArmeBruit` false true)
  (`self.UpdateAdditionalInformation`))

(fn `UserConstructionScript`
  (`parent.UserConstructionScript`)
  ;[1 1 1] Chargé ou non
  (if (`self.Loaded`)
    (set `self.Ammo` (defaults `/Game/JustATestAssets/Environnement/Usable/Items/Weapon/DistanceWeapon/Pistol1/Pistol1BP` (`self.AmmoType`)))
    (else
      (`SceneComponent.SetVisibility` (`self.Cartouche`) false false))))