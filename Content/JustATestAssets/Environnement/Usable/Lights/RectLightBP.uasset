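; RectLightBP is a usable light actor whose rect light brightness is set by a command sent to the actor.
; The SendCommandtoActor event converts its CommandId to a float and applies it directly as the RectLight intensity, so the ID doubles as the brightness value.
; It has no other active logic, as BeginPlay, overlap and Tick are disabled and the construction script only calls the parent.
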(event `/Game/JustATestAssets/Environnement/Usable/Activator/ActivableInterface.SendCommandToActor`
  (params (CommandId :type Integer))
  ;[1 1 1] Set intensity
  (`LightComponent.SetIntensity` (`self.RectLight`) (`KismetMathLibrary.Conv_IntToDouble` CommandId)))

(fn `UserConstructionScript`
  (`parent.UserConstructionScript`))