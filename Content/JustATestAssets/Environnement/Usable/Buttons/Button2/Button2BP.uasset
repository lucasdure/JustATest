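; Button2BP is a usable button with a press animation and a screen that displays an open/close state.
; At BeginPlay it creates a dynamic material instance for the screen slot of its static mesh.
; ActivatorFXorAnimation plays a timeline that slides a second mesh along relative X.
; SendStatetoActor swaps the screen's Diffuse texture to show closed, closing, opened or opening according to the received state.
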(event `self.ReceiveBeginPlay`
  (bind _staticmesh (`self.StaticMesh`))
  (`parent.ReceiveBeginPlay`)
  ;[1 1 1] Instance of screen
  (bind _returnvalue (`PrimitiveComponent.CreateDynamicMaterialInstance` _staticmesh 1 (`PrimitiveComponent.GetMaterial` _staticmesh 1) "None"))
  (bind _output_get (set `self.ScreenMat` _returnvalue))
  (`PrimitiveComponent.SetMaterial` (`self.StaticMesh`) 1 _output_get))

(event `self.ActivatorFXOrAnimation`
  ;[1 1 1] ButtonAnimation
  (bind (_direction _relativex) (`Timeline|Location` :!via `PlayFromStart`)
    (:`Update`
      (`SceneComponent.K2_SetRelativeLocation` (`self.StaticMesh1`) (`KismetMathLibrary.MakeVector` _relativex) false false))))

(event `/Game/JustATestAssets/Environnement/Usable/Activator/ActivableInterface.SendStateToActor`
  (params (State :type Integer))
  ;[1 1 1] Changes screen
  (`MaterialInstanceDynamic.SetTextureParameterValue` (`self.ScreenMat`) "Diffuse" (select `int` State :`0` "/Game/JustATestAssets/Environnement/Usable/Buttons/Button2/ClosedScreen.ClosedScreen" :`1` "/Game/JustATestAssets/Environnement/Usable/Buttons/Button2/ClosingScreen.ClosingScreen" :`2` "/Game/JustATestAssets/Environnement/Usable/Buttons/Button2/OpenedScreen.OpenedScreen" :`3` "/Game/JustATestAssets/Environnement/Usable/Buttons/Button2/OpeningScreen.OpeningScreen" :!type "Texture Object Reference")))

(fn `UserConstructionScript`
  (`parent.UserConstructionScript`))