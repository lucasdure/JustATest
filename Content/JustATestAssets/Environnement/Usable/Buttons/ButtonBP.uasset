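; ButtonBP is a usable button that sends commands to a list of target actors when activated through ActivatorUsed or UseObject.
; If usable, optionally gated to server authority, it passes a DoOnce that resets immediately unless the button is single-use.
; It calls an empty ActivatorFXOrAnimation hook, plays a sound at its location, waits a configurable delay, then messages each target its command ID.
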(event `/Game/JustATestAssets/Environnement/Usable/Activator/ActivatorInterface.ActivatorUsed`
  ;[1 1 1] Send commands to actors
  (if (`self.Usable`) :!label _label
    (if (`self.ServerOnly`)
      (`/Engine/EditorBlueprintResources/ActorMacros.Switch Has Authority`
        (:`Authority`
          _)))
    (`/Engine/EditorBlueprintResources/StandardMacros.DoOnce` false :!label _label_2
      (:`Completed`
        (if (not (`self.UsableOnce`))
          (`|ExecutionSequence`
            (:`then_0`
              (goto _label_2 :!via `Reset`))
            (:`then_1`
              _)))
        (`self.ActivatorFXOrAnimation`)
        (`GameplayStatics.PlaySoundAtLocation` (`self.ButtonSound`) (`SceneComponent.K2_GetComponentLocation` (`self.DefaultSceneRoot`)) (struct) 1.0 1.0 0.0 null null null)
        (`KismetSystemLibrary.Delay` (`self.TimeToActive`))
        (for _array_element (`self.ListOfActorToCommand`)
          (message `/Game/JustATestAssets/Environnement/Usable/Activator/ActivableInterface.SendCommandToActor` (break `/Game/JustATestAssets/Environnement/Usable/Activator/CommandStruture` _array_element) (`.CommandId_5_0567DCA54BE6F84D074491A995DBB6FB` (break `/Game/JustATestAssets/Environnement/Usable/Activator/CommandStruture` _array_element))))))))

(event `/Game/JustATestAssets/Environnement/Pawns/Humans/InteractionEnvironment.UseObject`
  (params (HumanRef :type "/Game/JustATestAssets/Environnement/Pawns/Humans/ControlableCharacter Object Reference") (Bis :type Boolean) (Instant :type Boolean))
  ;[1 1 1] Send commands to actors
  (goto _label))

(event `ActivatorFXOrAnimation`)

(fn `UserConstructionScript`
  (`parent.UserConstructionScript`))