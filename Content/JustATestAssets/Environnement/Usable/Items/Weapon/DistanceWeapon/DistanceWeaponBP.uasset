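; Base ranged weapon item that fires projectiles and applies their impacts, with empty Unload, Reload and SpecialFx hooks.
; Fire spends ammo, updates HUD and aims the local player's shot by camera trace, falling back to camera rotation.
; Shots and impacts relay through Server and Multi events that skip the owning player, whose shot spawns immediately.
; Loaded state and ammo persist in inventory item data, while audio parameters select weapon sounds.
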(event `self.ReceiveTick`
  (params (DeltaSeconds :type "Float (single-precision)"))
  (`parent.ReceiveTick` DeltaSeconds))

(event `FireProjectileLocal`
  (params (`Projectile Location` :type "Vector Structure") (`Projectile Rotation` :type "Rotator Structure") (FromServer :type Boolean))
  (bind _weaponactivation (`self.WeaponActivation`))
  ;[1 1 1] FireWithWeapon
  (bind _returnvalue (`|SpawnActorFromClass` (`self.Projectile`) (`KismetMathLibrary.MakeTransform` `Projectile Location` `Projectile Rotation`) "AlwaysSpawn" "OverrideRootScale" null null))
  (set `/Game/JustATestAssets/Environnement/Usable/Items/Weapon/Projectiles/ProjectileBP.WeaponRef` self _returnvalue)
  (set `/Game/JustATestAssets/Environnement/Usable/Items/Weapon/Projectiles/ProjectileBP.OriginalActor` (`self.TemporaryHumanRef`) _returnvalue)
  (set `/Game/JustATestAssets/Environnement/Usable/Items/Weapon/Projectiles/ProjectileBP.FromServer` FromServer _returnvalue)
  (`self.SpecialFx`)
  (`AudioComponent.SetIntParameter` _weaponactivation "Type" (`self.ItemFireType`))
  (`AudioComponent.Play` _weaponactivation 0.0))

(event `Fire`
  (bind _returnvalue (`GameplayStatics.GetPlayerCameraManager` 0))
  (bind _returnvalue_2 (`SceneComponent.K2_GetComponentLocation` (`self.WeaponActivation`)))
  (bind _returnvalue_3 (`PlayerCameraManager.GetCameraLocation` _returnvalue))
  (bind _bodyscale_x (`KismetMathLibrary.BreakVector` (`/Game/JustATestAssets/Environnement/Pawns/Humans/ControlableCharacter.BodyScale` (`self.TemporaryHumanRef`))))
  (bind _healthmanaindicator (`/Game/JustATestAssets/HUD/Player/PlayerHud.HealthManaIndicator` (`/Game/JustATestAssets/Environnement/Pawns/Humans/ControlableCharacter.PlayerHud` (`self.TemporaryHumanRef`))))
  ;[1 1 1] FireWithWeapon
  (`/Engine/EditorBlueprintResources/StandardMacros.DecrementInt` (`self.Ammo`)
    (:`  `
      (`self.UpdateAdditionalInformation`)
      (if (== (`GameplayStatics.GetPlayerPawn` 0) (`self.TemporaryHumanRef`))
        (if (`self.LeftHandWeapon`)
          (`/Game/JustATestAssets/HUD/Player/HealthManaBar.UpdateLeftWeapon` _healthmanaindicator false)
          (else
            (`/Game/JustATestAssets/HUD/Player/HealthManaBar.UpdateRightWeapon` _healthmanaindicator false)))
        (bind (_outhit _returnvalue_4) (`KismetSystemLibrary.LineTraceSingle` _returnvalue_3 (+ _returnvalue_3 (* (`self.GetActorForwardVector` _returnvalue) 100000)) "TraceTypeQuery1" true))
        (`|ExecutionSequence`
          (:`then_0`
            (bind _returnvalue_5 (select `bool` (and _returnvalue_4 (> (`.Distance` (`GameplayStatics.BreakHitResult` _outhit)) (* 50 _bodyscale_x))) :`false` (`PlayerCameraManager.GetCameraRotation` _returnvalue) :`true` (`KismetMathLibrary.MakeRotFromX` (- (`.Location` (`GameplayStatics.BreakHitResult` _outhit)) _returnvalue_2))))
            (`self.FireProjectileLocal` _returnvalue_2 _returnvalue_5))
          (:`then_1`
            (`self.FireProjectileServer` _returnvalue_2 _returnvalue_5)))))))

(event `FireProjectileServer`
  (params (`Projectile Location` :type "Vector Structure") (`Projectile Rotation` :type "Rotator Structure"))
  ;[1 1 1] FireWithWeapon
  (`self.FireProjectileMulti` `Projectile Location` `Projectile Rotation`))

(event `FireProjectileMulti`
  (params (`Projectile Location` :type "Vector Structure") (`Projectile Rotation` :type "Rotator Structure"))
  ;[1 1 1] FireWithWeapon
  (if (not (== (`self.TemporaryHumanRef`) (`GameplayStatics.GetPlayerPawn` 0)))
    (`self.FireProjectileLocal` `Projectile Location` `Projectile Rotation` true)))

(event `Unload`
  ;[1 1 1] FireWithWeapon
)

(event `Reload`
  ;[1 1 1] FireWithWeapon
)

(event `SpecialFx`
  ;[1 1 1] FireWithWeapon
)

(event `ProjectileImpactLocal`
  (params (Hit :type "HitResult Structure") (Damages :type Integer) (Velocity :type "Vector Structure"))
  ;[1 1 1] GenerateImpact
  (bind _returnvalue (`|SpawnActorFromClass` "/Game/JustATestAssets/Environnement/Effect/ImpactEffect/ImpactEffectBP.ImpactEffectBP_C" (`KismetMathLibrary.MakeTransform` Hit_Location) "AlwaysSpawn" "OverrideRootScale" null null))
  (`/Game/JustATestAssets/Environnement/Effect/ImpactEffect/ImpactEffectBP.GenerateImpact` _returnvalue Hit_PhysMat Hit_Normal Hit_HitComponent Hit_HitBoneName)
  (message `/Game/JustATestAssets/Environnement/Pawns/Humans/InteractionEnvironment.ApplyEffectInterface` Hit_HitActor Damages Velocity Hit_HitBoneName false))

(event `/Game/JustATestAssets/Environnement/Usable/Items/Weapon/Projectile_OriginalActor.ProjectileImpact`
  (params (Hit :type "HitResult Structure") (Damages :type Integer) (Velocity :type "Vector Structure"))
  ;[1 1 1] GenerateImpact
  (`self.ProjectileImpactServer` Hit Damages Velocity))

(event `self.UpdateAdditionalInformation`
  (bind (_itemproperties_imageref _itemproperties_itemclass _itemproperties_iteminventoryposition _itemproperties_itemsize _itemproperties_shorcut _itemproperties_additionalinformation) (break `/Game/JustATestAssets/Environnement/Usable/Items/ItemPropertiesInventory` (`self.ItemProperties`)))
  (bind (_inventory_size _inventory_items) (break `/Game/JustATestAssets/Environnement/Pawns/Humans/Inventory` (`/Game/JustATestAssets/Environnement/Pawns/Humans/ControlableCharacter.Inventory` (`self.TemporaryHumanRef`))))
  ;[1 1 1] Update add info for gun
  (setmembers `/Game/JustATestAssets/Environnement/Usable/Items/ItemPropertiesInventory` :`StructRef` (`self.ItemProperties`) :`AdditionalInformation` (`|MakeArray` (`KismetMathLibrary.Conv_BoolToDouble` (`self.Loaded`)) (`KismetMathLibrary.Conv_IntToDouble` (`self.Ammo`))))
  (for (_array_element _array_index) _inventory_items
    (if (== (`.ItemInventoryPosition_14_F3E2699543AFA2F7C05F2489D68BDBD6` (break `/Game/JustATestAssets/Environnement/Usable/Items/ItemPropertiesInventory` _array_element)) _itemproperties_iteminventoryposition)
      (setmembers `/Game/JustATestAssets/Environnement/Usable/Items/ItemPropertiesInventory` :`StructRef` (`|GetArrayItem` _inventory_items _array_index) :`AdditionalInformation` _itemproperties_additionalinformation)
      (break))))

(event `ProjectileImpactServer`
  (params (Hit :type "HitResult Structure") (Damages :type Integer) (Velocity :type "Vector Structure"))
  ;[1 1 1] GenerateImpact
  (`self.ProjectileImpactMulti` Hit Damages Velocity))

(event `ProjectileImpactMulti`
  (params (Hit :type "HitResult Structure") (Damages :type Integer) (Velocity :type "Vector Structure"))
  ;[1 1 1] GenerateImpact
  (if (not (== (`GameplayStatics.GetPlayerPawn` 0) (`self.TemporaryHumanRef`)))
    (`self.ProjectileImpactLocal` Hit Damages Velocity)))

(event `self.UseAdditionalInformation`
  (params (AdditionalInformation :type "Array of Float (single-precision) (by ref)"))
  ;[1 1 1] Use add info
  (set `self.Loaded` (== (`|GetArrayItem` AdditionalInformation) 1.0))
  (set `self.Ammo` (`KismetMathLibrary.FTrunc` (`|GetArrayItem` AdditionalInformation 1))))

(fn `ArmeBruit`
  (params (Unload :type Boolean) (Reload :type Boolean) (NoAmmo :type Boolean))
  (bind _weaponinternsound (`self.WeaponInternSound`))
  (`AudioComponent.SetBoolParameter` _weaponinternsound "Unload" Unload)
  (`AudioComponent.SetBoolParameter` _weaponinternsound "Reload" Reload)
  (`AudioComponent.SetBoolParameter` _weaponinternsound "NoAmmo" NoAmmo)
  (`AudioComponent.Play` _weaponinternsound 0.0))

(fn `UserConstructionScript`
  (`parent.UserConstructionScript`)
  ;[1 1 1] Sound type
  (`AudioComponent.SetIntParameter` (`self.WeaponInternSound`) "Type" (`self.ItemFireType`)))