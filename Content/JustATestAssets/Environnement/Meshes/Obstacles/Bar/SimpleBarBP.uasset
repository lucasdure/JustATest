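; SimpleBarBP is a bar obstacle that ControlableCharacters can grab when falling or wall-running.
; Two trigger boxes track overlapping characters in separate lists, with Box1 flagging the up-bar case.
; Each tick, it calls GrimperBarre on eligible characters, passing the bar position, arrow rotation and box dimensions.
; GetPosition projects the character onto the bar's horizontal line, perpendicular to the arrow, at the mesh's height.
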(event `self.Box.OnComponentBeginOverlap`
  (params (OverlappedComponent :type "PrimitiveComponent Object Reference") (OtherActor :type "Actor Object Reference") (OtherComp :type "PrimitiveComponent Object Reference") (OtherBodyIndex :type Integer) (bFromSweep :type Boolean) (SweepResult :type "HitResult Structure (by ref)"))
  ;[1 1 1] Vérifier qui est dans la boite
  (bind _ascontrolable_character (cast `/Game/JustATestAssets/Environnement/Pawns/Humans/ControlableCharacter` OtherActor))
  (`KismetArrayLibrary.Array_Add` (`self.CharactersInBox`) _ascontrolable_character))

(event `self.Box1.OnComponentBeginOverlap`
  (params (OverlappedComponent :type "PrimitiveComponent Object Reference") (OtherActor :type "Actor Object Reference") (OtherComp :type "PrimitiveComponent Object Reference") (OtherBodyIndex :type Integer) (bFromSweep :type Boolean) (SweepResult :type "HitResult Structure (by ref)"))
  ;[1 1 1] Vérifier qui est dans la boite1
  (bind _ascontrolable_character (cast `/Game/JustATestAssets/Environnement/Pawns/Humans/ControlableCharacter` OtherActor))
  (`KismetArrayLibrary.Array_Add` (`self.CharactersInBox1`) _ascontrolable_character))

(event `self.Box1.OnComponentEndOverlap`
  (params (OverlappedComponent :type "PrimitiveComponent Object Reference") (OtherActor :type "Actor Object Reference") (OtherComp :type "PrimitiveComponent Object Reference") (OtherBodyIndex :type Integer))
  ;[1 1 1] Vérifier qui est dans la boite1
  (bind _ascontrolable_character (cast `/Game/JustATestAssets/Environnement/Pawns/Humans/ControlableCharacter` OtherActor))
  (`KismetArrayLibrary.Array_RemoveItem` (`self.CharactersInBox1`) _ascontrolable_character))

(event `self.Box.OnComponentEndOverlap`
  (params (OverlappedComponent :type "PrimitiveComponent Object Reference") (OtherActor :type "Actor Object Reference") (OtherComp :type "PrimitiveComponent Object Reference") (OtherBodyIndex :type Integer))
  ;[1 1 1] Vérifier qui est dans la boite
  (bind _ascontrolable_character (cast `/Game/JustATestAssets/Environnement/Pawns/Humans/ControlableCharacter` OtherActor))
  (`KismetArrayLibrary.Array_RemoveItem` (`self.CharactersInBox`) _ascontrolable_character))

(event `self.ReceiveTick`
  (params (DeltaSeconds :type "Float (single-precision)"))
  (bind _box1 (`self.Box1`))
  (bind _returnvalue (`SceneComponent.K2_GetComponentRotation` (`self.Arrow`)))
  (bind _returnvalue_2 (`SceneComponent.K2_GetComponentLocation` _box1))
  (bind (_boxextent_x _boxextent_y) (`KismetMathLibrary.BreakVector` (`BoxComponent.BoxExtent` (`self.Box`))))
  (bind (_boxextent_x_2 _boxextent_y_2) (`KismetMathLibrary.BreakVector` (`BoxComponent.BoxExtent` _box1)))
  (`|ExecutionSequence`
    (:`then_0`
      ;[1 1 1] Faire utiliser perso
      (for _array_element (`self.CharactersInBox`)
        (if (or (`NavMovementComponent.IsFalling` (`Character.CharacterMovement` _array_element)) (`/Game/JustATestAssets/Environnement/Pawns/Humans/ControlableCharacter.IsRunningWall` _array_element))
          (`/Game/JustATestAssets/Environnement/Pawns/Humans/ControlableCharacter.GrimperBarre` _array_element (`self.GetPosition` _array_element) _returnvalue false _boxextent_y_2 _returnvalue_2 _boxextent_y))))
    (:`then_1`
      (for _array_element_2 (`self.CharactersInBox1`)
        (if (or (`NavMovementComponent.IsFalling` (`Character.CharacterMovement` _array_element_2)) (`/Game/JustATestAssets/Environnement/Pawns/Humans/ControlableCharacter.IsRunningWall` _array_element_2))
          (`/Game/JustATestAssets/Environnement/Pawns/Humans/ControlableCharacter.GrimperBarre` _array_element_2 (`self.GetPosition` _array_element_2) _returnvalue true _boxextent_y_2 _returnvalue_2 _boxextent_y))))))

(fn `GetPosition`
  (params (Character :type "Character Object Reference"))
  (returns (Position :type "Vector Structure"))
  (locals (A :type "Vector2D Structure") (B :type "Vector2D Structure") (O :type "Vector2D Structure") (D :type "Vector2D Structure") (B1 :type "Float (double-precision)") (B2 :type "Float (double-precision)") (C2 :type "Vector2D Structure") (X :type "Float (double-precision)") (Y :type "Float (double-precision)"))
  (bind (_a_x _a_y) (`KismetMathLibrary.BreakVector2D` (`local.A`)))
  (bind (_d_x _d_y) (`KismetMathLibrary.BreakVector2D` (`local.D`)))
  (bind (_b_x _b_y) (`KismetMathLibrary.BreakVector2D` (`local.B`)))
  (bind (_c2_x _c2_y) (`KismetMathLibrary.BreakVector2D` (`local.C2`)))
  (bind (_c2_x_2 _c2_y_2) (`KismetMathLibrary.BreakVector2D` (`local.C2`)))
  (bind (_d_x_2 _d_y_2) (`KismetMathLibrary.BreakVector2D` (`local.D`)))
  (bind (_d_x_3 _d_y_3) (`KismetMathLibrary.BreakVector2D` (`local.D`)))
  (bind _d (`local.D`))
  (bind (_returnvalue_x _returnvalue_y _returnvalue_z) (`KismetMathLibrary.BreakVector` (`SceneComponent.K2_GetComponentLocation` (`self.StaticMesh`))))
  (bind (_returnvalue_x_2 _returnvalue_y_2) (`KismetMathLibrary.BreakVector` (`SceneComponent.K2_GetComponentLocation` (`Character.CapsuleComponent` Character))))
  (bind (_returnvalue_x_3 _returnvalue_y_3) (`KismetMathLibrary.BreakVector` (`SceneComponent.K2_GetComponentLocation` (`self.StaticMesh`))))
  (bind (_returnvalue_x_4 _returnvalue_y_4) (`KismetMathLibrary.BreakVector` (`KismetMathLibrary.Cross_VectorVector` (`SceneComponent.GetForwardVector` (`self.Arrow`)) (0.0 0.0 1.0))))
  (set `local.A` (`KismetMathLibrary.MakeVector2D` _returnvalue_x_3 _returnvalue_y_3))
  (bind _output_get (set `local.B` (`KismetMathLibrary.MakeVector2D` _returnvalue_x_2 _returnvalue_y_2)))
  (set `local.O` (- _output_get (`local.A`)))
  (set `local.D` (`KismetMathLibrary.MakeVector2D` _returnvalue_x_4 _returnvalue_y_4))
  (set `local.C2` (- (- (`local.B`) (`local.A`)) (* (`local.D`) (/ (`KismetMathLibrary.DotProduct2D` (`local.O`) _d) (`KismetMathLibrary.DotProduct2D` _d _d)))))
  (set `local.B1` (- _a_y (* _a_x (/ _d_y_2 _d_x_2))))
  (set `local.B2` (- _b_y (* _b_x (/ _c2_y_2 _c2_x_2))))
  (set `local.X` (/ (- (`local.B2`) (`local.B1`)) (- (/ _d_y_3 _d_x_3) (/ _c2_y _c2_x))))
  (set `local.Y` (+ (* (`local.X`) (/ _d_y _d_x)) (`local.B1`)))
  (return (`KismetMathLibrary.MakeVector` (`local.X`) (`local.Y`) _returnvalue_z)))

(fn `UserConstructionScript`)