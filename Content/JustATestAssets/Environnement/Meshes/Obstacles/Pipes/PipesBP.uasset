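; Climbable pipe obstacle that airborne ControlableCharacters can grab onto.
; A box trigger tracks the characters inside it, and Tick checks each one that is falling.
; If the character faces the pipe on the horizontal plane, is not already climbing and is between the UpPipe and DownPipe heights, it calls the character's GrabPipes.
; That call passes the arrow position, mesh rotation and both end markers.
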(event `self.Box.OnComponentBeginOverlap`
  (params (OverlappedComponent :type "PrimitiveComponent Object Reference") (OtherActor :type "Actor Object Reference") (OtherComp :type "PrimitiveComponent Object Reference") (OtherBodyIndex :type Integer) (bFromSweep :type Boolean) (SweepResult :type "HitResult Structure (by ref)"))
  ;[1 1 1] Vérifier qui est dans la boite
  (bind _ascontrolable_character (cast `/Game/JustATestAssets/Environnement/Pawns/Humans/ControlableCharacter` OtherActor))
  (`KismetArrayLibrary.Array_Add` (`self.CharactersInBox`) _ascontrolable_character))

(event `self.Box.OnComponentEndOverlap`
  (params (OverlappedComponent :type "PrimitiveComponent Object Reference") (OtherActor :type "Actor Object Reference") (OtherComp :type "PrimitiveComponent Object Reference") (OtherBodyIndex :type Integer))
  ;[1 1 1] Vérifier qui est dans la boite
  (bind _ascontrolable_character (cast `/Game/JustATestAssets/Environnement/Pawns/Humans/ControlableCharacter` OtherActor))
  (`KismetArrayLibrary.Array_RemoveItem` (`self.CharactersInBox`) _ascontrolable_character))

(event `self.ReceiveTick`
  (params (DeltaSeconds :type "Float (single-precision)"))
  (bind (_returnvalue_x _returnvalue_y _returnvalue_z) (`KismetMathLibrary.BreakVector` (`SceneComponent.K2_GetComponentLocation` (`self.DownPipe`))))
  (bind (_returnvalue_x_2 _returnvalue_y_2 _returnvalue_z_2) (`KismetMathLibrary.BreakVector` (`SceneComponent.K2_GetComponentLocation` (`self.UpPipe`))))
  (`|ExecutionSequence`
    (:`then_0`
      ;[1 1 1] Faire utiliser perso
      (for _array_element (`self.CharactersInBox`)
        (if (`NavMovementComponent.IsFalling` (`Character.CharacterMovement` _array_element))
          (bind _capsulecomponent (`Character.CapsuleComponent` _array_element))
          (bind (_returnvalue_x_3 _returnvalue_y_3) (`KismetMathLibrary.BreakVector` (`SceneComponent.GetForwardVector` _capsulecomponent)))
          (bind _returnvalue (`SceneComponent.K2_GetComponentLocation` _capsulecomponent))
          (bind (_returnvalue_x_4 _returnvalue_y_4) (`KismetMathLibrary.BreakVector` (- (`SceneComponent.K2_GetComponentLocation` (`self.StaticMesh`)) _returnvalue)))
          (bind _z (.z _returnvalue))
          (if (and (> (`KismetMathLibrary.Dot_VectorVector` (`KismetMathLibrary.MakeVector` _returnvalue_x_3 _returnvalue_y_3) (`KismetMathLibrary.MakeVector` _returnvalue_x_4 _returnvalue_y_4)) 0.0) (not (`/Game/JustATestAssets/Environnement/Pawns/Humans/ControlableCharacter.ClimbingPipe` _array_element)) (< _z _returnvalue_z_2) (> _z _returnvalue_z))
            (`/Game/JustATestAssets/Environnement/Pawns/Humans/ControlableCharacter.GrabPipes` _array_element (`SceneComponent.K2_GetComponentLocation` (`self.Arrow`)) (`SceneComponent.K2_GetComponentRotation` (`self.StaticMesh`)) (`self.UpPipe`) (`self.DownPipe`))))))))

(fn `UserConstructionScript`)