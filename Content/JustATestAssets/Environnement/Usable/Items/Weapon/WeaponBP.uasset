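; WeaponBP is a weapon Blueprint that supplies impact decal selection and an FX hook, apparently as a base for specific weapons.
; GetDecalClassRotation picks a bullet-hole decal class by index, with only concrete, metal and plastic filled in, and derives its rotation from the surface normal.
; TriggerFX is an empty event with a Stop parameter, and BeginPlay, overlap and Tick are disabled stubs.
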(event `TriggerFX`
  (params (Stop :type Boolean)))

(fn `GetDecalClassRotation`
  (params (Index :type Integer) (Normal :type "Vector Structure"))
  (returns (ReturnValue :type "Actor Class Reference") (Rotation :type "Rotator Structure"))
  (return (select `int` Index :`0` null :`1` null :`2` "/Game/JustATestAssets/Environnement/Effect/ImpactEffect/ImpactTexture/DecalHoleConcrete.DecalHoleConcrete_C" :`3` null :`4` null :`5` null :`6` "/Game/JustATestAssets/Environnement/Effect/ImpactEffect/ImpactTexture/DecalHoleMetal.DecalHoleMetal_C" :`7` "/Game/JustATestAssets/Environnement/Effect/ImpactEffect/ImpactTexture/DecalHolePlastic.DecalHolePlastic_C" :`8` null :`9` null :`10` null :`11` null :`12` null :!type "Actor Class Reference") (`KismetMathLibrary.MakeRotFromX` Normal)))

(fn `UserConstructionScript`
  (`parent.UserConstructionScript`))