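; ImpactEffectBP is an actor that produces projectile impact effects through its GenerateImpact event.
; It looks up the impact type in PhysList, then spawns sound and particle actors configured with that result.
; The same lookup selects a concrete, metal or plastic hole decal, oriented to the normal and attached to the hit component.
; Hits on a ControlableCharacter also call Paint on its head mesh or main clothes, depending on the bone.
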(event `GenerateImpact`
  (params (ImpactType :type "PhysicalMaterial Object Reference") (Normal :type "Vector Structure (by ref)") (ComponentTargeted :type "SceneComponent Object Reference") (BoneTargeted :type Name))
  (bind _returnvalue (`ActorComponent.GetOwner` ComponentTargeted))
  (bind _returnvalue_2 (`KismetArrayLibrary.Array_Find` (`self.PhysList`) ImpactType))
  ;[1 1 1] ProjectileImpact
  (bind _returnvalue_3 (`|SpawnActorFromClass` "/Game/JustATestAssets/Environnement/Effect/ImpactEffect/ImpactSound/ImpactSoundBP.ImpactSoundBP_C" (`KismetMathLibrary.MakeTransform` (`SceneComponent.K2_GetComponentLocation` (`self.DefaultSceneRoot`))) "AlwaysSpawn" "OverrideRootScale" null null))
  (`/Game/JustATestAssets/Environnement/Effect/ImpactEffect/ImpactSound/ImpactSoundBP.ImpactSound` _returnvalue_3 _returnvalue_2)
  (bind _returnvalue_4 (`|SpawnActorFromClass` "/Game/JustATestAssets/Environnement/Effect/ImpactEffect/ImpactParticle/ImpactParticleBP.ImpactParticleBP_C" (`KismetMathLibrary.MakeTransform` (`SceneComponent.K2_GetComponentLocation` (`self.DefaultSceneRoot`))) "AlwaysSpawn" "OverrideRootScale" null null))
  (`/Game/JustATestAssets/Environnement/Effect/ImpactEffect/ImpactParticle/ImpactParticleBP.SetParticles` _returnvalue_4 _returnvalue_2)
  (bind _returnvalue_5 (`|SpawnActorFromClass` (select `int` _returnvalue_2 :`0` null :`1` null :`2` "/Game/JustATestAssets/Environnement/Effect/ImpactEffect/ImpactTexture/DecalHoleConcrete.DecalHoleConcrete_C" :`3` null :`4` null :`5` null :`6` "/Game/JustATestAssets/Environnement/Effect/ImpactEffect/ImpactTexture/DecalHoleMetal.DecalHoleMetal_C" :`7` "/Game/JustATestAssets/Environnement/Effect/ImpactEffect/ImpactTexture/DecalHolePlastic.DecalHolePlastic_C" :`8` null :`9` null :`10` null :`11` null :`12` null :!type "Actor Class Reference") (`KismetMathLibrary.MakeTransform` (`SceneComponent.K2_GetComponentLocation` (`self.DefaultSceneRoot`)) (`KismetMathLibrary.MakeRotFromX` Normal)) "AlwaysSpawn" "OverrideRootScale" null null))
  (`/Engine/EditorBlueprintResources/StandardMacros.IsValid` _returnvalue_5
    (:`Is Valid`
      (`self.K2_AttachToComponent` _returnvalue_5 ComponentTargeted "None" "KeepWorld" "KeepWorld" "KeepWorld" true)
      (`/Engine/EditorBlueprintResources/StandardMacros.IsValid` _returnvalue
        (:`Is Valid`
          _)))
    (:`Is Not Valid`
      _))
  (bind _ascontrolable_character (cast `/Game/JustATestAssets/Environnement/Pawns/Humans/ControlableCharacter` _returnvalue))
  (`/Game/JustATestAssets/Environnement/Pawns/Humans/ControlableCharacter.Paint` _ascontrolable_character (`SceneComponent.K2_GetComponentLocation` (`self.DefaultSceneRoot`)) 5.0 (select `bool` (== BoneTargeted "head") :`false` (`/Game/JustATestAssets/Environnement/Pawns/Humans/ControlableCharacter.MainClothes` _ascontrolable_character) :`true` (`Character.Mesh` _ascontrolable_character) :!type "ActorComponent Object Reference")))

(fn `UserConstructionScript`)