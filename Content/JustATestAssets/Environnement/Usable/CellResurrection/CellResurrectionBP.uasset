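; Resurrection cell that revives ghost players: on the server, a GhostPawn overlapping its sphere is resurrected just above the cell mesh.
; The construction script registers both child doors and the cell with a child TriggerDetection for commands.
; When commanded, it turns the left door light red and plays smoke; Tick restores green and sphere collision once both doors close.
; A multicast-named state event can disable the sphere.
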(event `self.ReceiveTick`
  (params (DeltaSeconds :type "Float (single-precision)"))
  ;[1 1 1] Peut ressuciter de nouveau
  (if (and (`self.CellIsOpening`) (`/Game/JustATestAssets/Environnement/Usable/Doors/DoorBP.IsClosed` (`self.DoorLeftRef`)) (`/Game/JustATestAssets/Environnement/Usable/Doors/DoorBP.IsClosed` (`self.DoorRightLeft`)))
    (set `self.CellIsOpening` false)
    (`PrimitiveComponent.SetMaterial` (`/Game/JustATestAssets/Environnement/Usable/Doors/DoorBP.Door` (`self.DoorLeftRef`)) 1 "/Game/JustATestAssets/Environnement/Materials/SimpleMaterials/EmissiveColor/GreenLight.GreenLight")
    (`PrimitiveComponent.SetCollisionEnabled` (`self.Sphere`) "QueryOnly")))

(event `ChangeActorStateMulti`
  (params (State :type Integer))
  ;[1 1 1] Change Cell State Network
  (switch `int` State
    (:`0`
      (`PrimitiveComponent.SetCollisionEnabled` (`self.Sphere`) "NoCollision"))))

(event `/Game/JustATestAssets/GameModes/DebugMode/NetworkState.ChangeActorState`
  (params (State :type Integer))
  ;[1 1 1] Change Cell State Network
  (`self.ChangeActorStateMulti` State))

(event `self.Sphere.OnComponentBeginOverlap`
  (params (OverlappedComponent :type "PrimitiveComponent Object Reference") (OtherActor :type "Actor Object Reference") (OtherComp :type "PrimitiveComponent Object Reference") (OtherBodyIndex :type Integer) (bFromSweep :type Boolean) (SweepResult :type "HitResult Structure (by ref)"))
  ;[1 1 1] Resurrection
  (`/Engine/EditorBlueprintResources/ActorMacros.Switch Has Authority`
    (:`Authority`
      (bind _asghost_pawn (cast `/Game/JustATestAssets/Environnement/Pawns/GhostPawn` OtherActor))
      (set `self.RefGhost` _asghost_pawn)
      (bind _ashuman_controler (cast `/Game/JustATestAssets/GameModes/DebugMode/HumanControler` (`Pawn.GetController` _asghost_pawn)))
      (`/Game/JustATestAssets/Environnement/Pawns/GhostPawn.Resurrection` (`self.RefGhost`) null _ashuman_controler (`KismetMathLibrary.MakeTransform` (+ (`SceneComponent.K2_GetComponentLocation` (`self.StaticMesh`)) (0.0 0.0 130.0)) (`SceneComponent.K2_GetComponentRotation` (`self.StaticMesh`)))))))

(event `/Game/JustATestAssets/Environnement/Usable/Activator/ActivableInterface.SendCommandToActor`
  (params (CommandId :type Integer))
  (switch `int` CommandId
    (:`0`
      ;[1 1 1] Ne peux plus ressuciter avant fermeture
      (`PrimitiveComponent.SetMaterial` (`/Game/JustATestAssets/Environnement/Usable/Doors/DoorBP.Door` (`self.DoorLeftRef`)) 1 "/Game/JustATestAssets/Environnement/Materials/SimpleMaterials/EmissiveColor/RedLight.RedLight")
      (if (not (`self.CellIsOpening`))
        (`ActorComponent.Activate` (`self.SmokeCell`) true)
        (`ActorComponent.Activate` (`self.SmokeCellFloor`) true)
        (`KismetSystemLibrary.Delay` 0.2)
        (set `self.CellIsOpening` true)))))

(fn `UserConstructionScript`
  (bind _doorleftref (`self.DoorLeftRef`))
  (bind _childactor (`ChildActorComponent.ChildActor` (`self.DoorRight`)))
  (bind _childactor_2 (`ChildActorComponent.ChildActor` (`self.DoorLeft`)))
  (`|ExecutionSequence`
    (:`then_0`
      (bind _astrigger_detection (cast `/Game/JustATestAssets/Environnement/Usable/Trigger/TriggerDetection` (`ChildActorComponent.ChildActor` (`self.Trigger`))))
      (bind _listofactortocommand (`/Game/JustATestAssets/Environnement/Usable/Activator/ActivatorBP.ListOfActorToCommand` _astrigger_detection))
      (`KismetArrayLibrary.Array_Add` _listofactortocommand (make `/Game/JustATestAssets/Environnement/Usable/Activator/CommandStruture` _childactor_2 1))
      (`KismetArrayLibrary.Array_Add` _listofactortocommand (make `/Game/JustATestAssets/Environnement/Usable/Activator/CommandStruture` _childactor 1))
      (`KismetArrayLibrary.Array_Add` _listofactortocommand (make `/Game/JustATestAssets/Environnement/Usable/Activator/CommandStruture` self))
      (bind _listofactortouncommand (`/Game/JustATestAssets/Environnement/Usable/Activator/ActivatorBP.ListOfActorToUncommand` _astrigger_detection))
      (`KismetArrayLibrary.Array_Add` _listofactortouncommand (make `/Game/JustATestAssets/Environnement/Usable/Activator/CommandStruture` _childactor_2 2))
      (`KismetArrayLibrary.Array_Add` _listofactortouncommand (make `/Game/JustATestAssets/Environnement/Usable/Activator/CommandStruture` _childactor 2))
      (`KismetArrayLibrary.Array_Add` _listofactortouncommand (make `/Game/JustATestAssets/Environnement/Usable/Activator/CommandStruture` self 1)))
    (:`then_1`
      (bind _ascell_door_left_bp (cast `/Game/JustATestAssets/Environnement/Usable/CellResurrection/CellDoorLeftBP` (`ChildActorComponent.ChildActor` (`self.DoorLeft`))))
      (set `self.DoorLeftRef` _ascell_door_left_bp))
    (:`then_2`
      (bind _ascell_door_right_bp (cast `/Game/JustATestAssets/Environnement/Usable/CellResurrection/CellDoorRightBP` (`ChildActorComponent.ChildActor` (`self.DoorRight`))))
      (set `self.DoorRightLeft` _ascell_door_right_bp))
    (:`then_3`
      (if (not (`self.On`))
        (set `/Game/JustATestAssets/Environnement/Usable/Doors/DoorBP.On` false _doorleftref)
        (`PrimitiveComponent.SetMaterial` (`/Game/JustATestAssets/Environnement/Usable/Doors/DoorBP.Door` _doorleftref) 1 "/Game/JustATestAssets/Environnement/Materials/SimpleMaterials/SimpleColor/Black.Black")))))