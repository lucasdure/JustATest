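; Base-style melee weapon Blueprint that applies damage and impact feedback when a hit is reported through ApplyWeaponEffect.
; It spawns an ImpactEffectBP at the hit position and calls GenerateImpact with the physical material, normal, component and bone.
; It then sends damage and an impulse along SceneRef's right vector to the target through an interface message.
; BeginPlay and the construction script only call the parent.
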(event `self.ReceiveBeginPlay`
  (`parent.ReceiveBeginPlay`))

(event `/Game/JustATestAssets/Environnement/Pawns/Humans/InteractionEnvironment.ApplyWeaponEffect`
  (params (WeaponTarget :type "Actor Object Reference") (Position :type "Vector Structure") (PhysicalMat :type "PhysicalMaterial Object Reference") (BoneName :type Name) (Normal :type "Vector Structure") (ComponentRef :type "SceneComponent Object Reference"))
  ;[1 1 1] Apply effect
  (bind _returnvalue (`|SpawnActorFromClass` "/Game/JustATestAssets/Environnement/Effect/ImpactEffect/ImpactEffectBP.ImpactEffectBP_C" (`KismetMathLibrary.MakeTransform` Position) "AlwaysSpawn" "OverrideRootScale" null null))
  (`/Game/JustATestAssets/Environnement/Effect/ImpactEffect/ImpactEffectBP.GenerateImpact` _returnvalue PhysicalMat Normal ComponentRef BoneName)
  (message `/Game/JustATestAssets/Environnement/Pawns/Humans/InteractionEnvironment.ApplyEffectInterface` WeaponTarget (`self.Damage`) (* (`SceneComponent.GetRightVector` (`self.SceneRef`)) (`self.Impulse`)) BoneName false))

(fn `UserConstructionScript`
  (`parent.UserConstructionScript`))