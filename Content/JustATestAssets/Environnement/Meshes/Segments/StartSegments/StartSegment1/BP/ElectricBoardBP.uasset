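; Electric board actor with a child lever and power cell slot, whose indicator lights show on, off or missing-cell state.
; Construction passes command lists to the lever, sets it for the On state, and blocks it while the cell is missing, linking the slot back to the board.
; A timeline flickers the yellow light until command 0 installs the cell and unlocks the lever; commands 1 and 2 switch green and red.
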(event `Light2Flickering`
  (params (Stop :type Boolean))
  ;[1 1 1] FlickeringEvent
  (if Stop
    (bind (_direction _flickvalue) (`Timeline|Flicker` :!via `Stop` :!label _label)
      (:`Update`
        (`self.SetFlicker` _flickvalue)))
    (else
      (goto _label :!via `PlayFromStart`))))

(event `self.ReceiveBeginPlay`
  (`parent.ReceiveBeginPlay`)
  ;[1 1 1] Start flickering if no cell
  (if (`self.MissingCell`)
    (`self.Light2Flickering` false)))

(event `/Game/JustATestAssets/Environnement/Usable/Activator/ActivableInterface.SendCommandToActor`
  (params (CommandId :type Integer))
  (bind _staticmesh (`self.StaticMesh`))
  (bind _staticmesh_2 (`self.StaticMesh`))
  (switch `int` CommandId
    (:`0`
      ;[1 1 1] ElectricBoard Activated
      (set `self.MissingCell` false)
      (if (`self.On`)
        (`PrimitiveComponent.SetMaterial` _staticmesh 2 "/Game/JustATestAssets/Environnement/Materials/SimpleMaterials/EmissiveColor/GreenLight.GreenLight")
        (else
          (`PrimitiveComponent.SetMaterial` _staticmesh 4 "/Game/JustATestAssets/Environnement/Materials/SimpleMaterials/EmissiveColor/RedLight.RedLight")))
      (`SceneComponent.SetVisibility` (`self.Cell`) true false)
      (`PrimitiveComponent.SetCollisionEnabled` (`/Game/JustATestAssets/Environnement/Usable/Doors/DoorBP.Door` (`self.LeverRef`)) "QueryOnly")
      (`self.Light2Flickering` true)
      (`PrimitiveComponent.SetMaterial` (`self.StaticMesh`) 3 "/Game/JustATestAssets/Environnement/Materials/SimpleMaterials/SimpleColor/Black.Black"))
    (:`1`
      ;[1 1 1] Change lighs of elec board
      (`PrimitiveComponent.SetMaterial` _staticmesh_2 2 "/Game/JustATestAssets/Environnement/Materials/SimpleMaterials/EmissiveColor/GreenLight.GreenLight")
      (`PrimitiveComponent.SetMaterial` _staticmesh_2 4 "/Game/JustATestAssets/Environnement/Materials/SimpleMaterials/SimpleColor/Black.Black"))
    (:`2`
      (`PrimitiveComponent.SetMaterial` _staticmesh_2 4 "/Game/JustATestAssets/Environnement/Materials/SimpleMaterials/EmissiveColor/RedLight.RedLight")
      (`PrimitiveComponent.SetMaterial` _staticmesh_2 2 "/Game/JustATestAssets/Environnement/Materials/SimpleMaterials/SimpleColor/Black.Black"))))

(fn `SetFlicker`
  (params (FlickerValue :type "Float (double-precision)"))
  (bind _light2black (`self.Light2Black`))
  (bind _staticmesh (`self.StaticMesh`))
  (if (< FlickerValue 0.0)
    (if (not _light2black)
      (`PrimitiveComponent.SetMaterial` _staticmesh 3 "/Game/JustATestAssets/Environnement/Materials/SimpleMaterials/SimpleColor/Black.Black")
      (set `self.Light2Black` true))
    (elif _light2black
      (`PrimitiveComponent.SetMaterial` _staticmesh 3 "/Game/JustATestAssets/Environnement/Materials/SimpleMaterials/EmissiveColor/YellowLight10.YellowLight10")
      (set `self.Light2Black` false))))

(fn `UserConstructionScript`
  (bind _staticmesh (`self.StaticMesh`))
  (bind _leverref (`self.LeverRef`))
  (`parent.UserConstructionScript`)
  (`|ExecutionSequence`
    (:`then_0`
      ;[1 1 1] Set list of actorToCommand
      (bind _aslever_board_bp (cast `/Game/JustATestAssets/Environnement/Meshes/Segments/StartSegments/StartSegment1/BP/LeverBoardBP` (`ChildActorComponent.ChildActor` (`self.Levier`))))
      (bind _output_get (set `self.LeverRef` _aslever_board_bp))
      (set `/Game/JustATestAssets/Environnement/Usable/Doors/DoorBP.ListOfActorToCommand` (`self.ActorsToCommand`) _output_get)
      (set `/Game/JustATestAssets/Environnement/Usable/Doors/DoorBP.ListOfActorToUncommand` (`self.ActorsToUncommand`) _output_get))
    (:`then_1`
      ;[1 1 1] SetLights
      (if (`self.MissingCell`)
        ;[1 1 1] Hide cell if no cell
        (`SceneComponent.SetVisibility` (`self.Cell`) false false)
        ;[1 1 1] Player can't use lever
        (`PrimitiveComponent.SetCollisionEnabled` (`/Game/JustATestAssets/Environnement/Usable/Doors/DoorBP.Door` (`self.LeverRef`)) "NoCollision")
        ;[1 1 1] Set ElectricBoardRef in emplacement cell
        (bind _asemplacement_cell (cast `/Game/JustATestAssets/Environnement/Meshes/Segments/StartSegments/StartSegment1/BP/EmplacementCell` (`ChildActorComponent.ChildActor` (`self.EmplacementCell`))))
        (set `/Game/JustATestAssets/Environnement/Meshes/Segments/StartSegments/StartSegment1/BP/EmplacementCell.ParentClass` self _asemplacement_cell)
        (else
          (if (`self.On`)
            (`PrimitiveComponent.SetMaterial` _staticmesh 2 "/Game/JustATestAssets/Environnement/Materials/SimpleMaterials/EmissiveColor/GreenLight.GreenLight")
            (else
              (`PrimitiveComponent.SetMaterial` _staticmesh 4 "/Game/JustATestAssets/Environnement/Materials/SimpleMaterials/EmissiveColor/RedLight.RedLight")))
          ;[1 1 1] Remove collision of emplacementCell
          (bind _asemplacement_cell_2 (cast `/Game/JustATestAssets/Environnement/Meshes/Segments/StartSegments/StartSegment1/BP/EmplacementCell` (`ChildActorComponent.ChildActor` (`self.EmplacementCell`))))
          (`PrimitiveComponent.SetCollisionEnabled` (`/Game/JustATestAssets/Environnement/Meshes/Segments/StartSegments/StartSegment1/BP/EmplacementCell.Sphere` _asemplacement_cell_2) "NoCollision"))))
    (:`then_2`
      ;[1 1 1] Change lever position
      (if (`self.On`)
        (set `/Game/JustATestAssets/Environnement/Usable/Doors/DoorBP.IsOpen` true _leverref)
        (set `/Game/JustATestAssets/Environnement/Usable/Doors/DoorBP.IsClosed` false _leverref)
        (`SceneComponent.K2_SetRelativeRotation` (`/Game/JustATestAssets/Environnement/Usable/Doors/DoorBP.Door` _leverref) (`/Game/JustATestAssets/Environnement/Usable/Doors/DoorBP.AimRotation` _leverref) false false)))))