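; AmmoBP is a usable inventory item for weapon ammunition that keeps its Ammo count in the item's generic AdditionalInformation float array.
; UpdateAdditionalInformation writes the count into ItemProperties, then copies it to the entry in TemporaryHumanRef's inventory with a matching ItemInventoryPosition.
; UseAdditionalInformation does the reverse, restoring Ammo by truncating the first array element to an integer.
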(event `self.UpdateAdditionalInformation`
  (bind (_itemproperties_imageref _itemproperties_itemclass _itemproperties_iteminventoryposition _itemproperties_itemsize _itemproperties_shorcut _itemproperties_additionalinformation) (break `/Game/JustATestAssets/Environnement/Usable/Items/ItemPropertiesInventory` (`self.ItemProperties`)))
  (bind (_inventory_size _inventory_items) (break `/Game/JustATestAssets/Environnement/Pawns/Humans/Inventory` (`/Game/JustATestAssets/Environnement/Pawns/Humans/ControlableCharacter.Inventory` (`self.TemporaryHumanRef`))))
  ;[1 1 1] Update add info for ammo
  (setmembers `/Game/JustATestAssets/Environnement/Usable/Items/ItemPropertiesInventory` :`StructRef` (`self.ItemProperties`) :`AdditionalInformation` (`|MakeArray` (`KismetMathLibrary.Conv_IntToDouble` (`self.Ammo`))))
  (for (_array_element _array_index) _inventory_items
    (if (== (`.ItemInventoryPosition_14_F3E2699543AFA2F7C05F2489D68BDBD6` (break `/Game/JustATestAssets/Environnement/Usable/Items/ItemPropertiesInventory` _array_element)) _itemproperties_iteminventoryposition)
      (setmembers `/Game/JustATestAssets/Environnement/Usable/Items/ItemPropertiesInventory` :`StructRef` (`|GetArrayItem` _inventory_items _array_index) :`AdditionalInformation` _itemproperties_additionalinformation)
      (break))))

(event `self.UseAdditionalInformation`
  (params (AdditionalInformation :type "Array of Float (single-precision) (by ref)"))
  ;[1 1 1] Use add info
  (set `self.Ammo` (`KismetMathLibrary.FTrunc` (`|GetArrayItem` AdditionalInformation))))

(fn `UserConstructionScript`
  (`parent.UserConstructionScript`))