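; Base pickup item that humans store in a grid inventory or equip in their hands, with override hooks for child items.
; On authority, UseObject finds free grid cells or a hand slot, stowing held items if needed, then records the item.
; Equipping attaches the mesh to one or both hands and updates animation and HUD.
; Hard hits play speed-scaled sounds and apply damage and knockdown, predicted by the owner and relayed through server and multicast events.
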(event `/Game/JustATestAssets/Environnement/Pawns/Humans/InteractionEnvironment.UseObject`
  (params (HumanRef :type "/Game/JustATestAssets/Environnement/Pawns/Humans/ControlableCharacter Object Reference") (Bis :type Boolean) (Instant :type Boolean))
  (bind _itemproperties (`self.ItemProperties`))
  (bind _temporaryhumanref (`self.TemporaryHumanRef`))
  (bind _inventory (`/Game/JustATestAssets/Environnement/Pawns/Humans/ControlableCharacter.Inventory` (`self.TemporaryHumanRef`)))
  (bind (_size _items) (break `/Game/JustATestAssets/Environnement/Pawns/Humans/Inventory` _inventory))
  ;[1 1 1] Mettre objet dans inventaire
  (if (not (`self.IsTaken`))
    (`/Engine/EditorBlueprintResources/ActorMacros.Switch Has Authority`
      (:`Authority`
        (set `self.BisUse` Bis)
        (set `self.Instant` Instant)
        (set `self.TemporaryHumanRef` HumanRef)
        (if (`self.BisUse`)
          (bind (_placefinded _coordinates) (`self.TrouverPlaceEquipement` _temporaryhumanref))
          (if _placefinded
            (if (`self.ItemCooldown`) :!label _label
              (`KismetSystemLibrary.Delay` 0.0)
              (goto _label)
              (else
                (set `self.TemporaryCoordinates` _coordinates)
                (`self.UpdateAdditionalInformation`)
                (bind _structout (setmembers `/Game/JustATestAssets/Environnement/Usable/Items/ItemPropertiesInventory` :`StructRef` _itemproperties :`ItemInventoryPosition` _coordinates))
                (`KismetArrayLibrary.Array_Add` _items _structout)
                (set `/Game/JustATestAssets/Environnement/Pawns/Humans/ControlableCharacter.Inventory` _inventory (`self.TemporaryHumanRef`) :!label _label_2)
                (set `self.IsTaken` true)
                (`self.RamasserObjet` (`self.TemporaryHumanRef`)))))
          (else
            (bind (_pasdeplace _colonnes _lignes) (`self.TrouverPlaceInventaire` _temporaryhumanref))
            (if _pasdeplace
              (`self.UpdateAdditionalInformation`)
              (bind _structout_2 (setmembers `/Game/JustATestAssets/Environnement/Usable/Items/ItemPropertiesInventory` :`StructRef` _itemproperties :`ItemInventoryPosition` (`KismetMathLibrary.MakeVector2D` (`KismetMathLibrary.Conv_IntToDouble` _colonnes) (`KismetMathLibrary.Conv_IntToDouble` _lignes))))
              (`KismetArrayLibrary.Array_Add` _items _structout_2)
              (goto _label_2))))))))

(event `DestroyActorEvent`
  ;[1 1 1] Mettre objet dans inventaire
  (`self.K2_DestroyActor`))

(event `RamasserObjet`
  (params (HumanRef :type "/Game/JustATestAssets/Environnement/Pawns/Humans/ControlableCharacter Object Reference"))
  (bind _menupersoref (`/Game/JustATestAssets/Environnement/Pawns/Humans/ControlableCharacter.MenuPersoRef` (`self.TemporaryHumanRef`)))
  (bind _healthmanaindicator (`/Game/JustATestAssets/HUD/Player/PlayerHud.HealthManaIndicator` (`/Game/JustATestAssets/Environnement/Pawns/Humans/ControlableCharacter.PlayerHud` (`self.TemporaryHumanRef`))))
  ;[1 1 1] Mettre objet dans inventaire
  (bind _output_get (set `self.TemporaryHumanRef` HumanRef))
  (`self.SetOwner` _output_get)
  (if (not (`self.Instant`))
    (`self.MoveItem`)
    (`/Engine/EditorBlueprintResources/StandardMacros.IsValid` _menupersoref
      (:`Is Valid`
        (`/Game/JustATestAssets/HUD/Menu/CharacterHud/CharacterMainHud.Refresh` _menupersoref))
      (:`Is Not Valid`
        _)))
  (if (`self.BisUse`)
    (`KismetSystemLibrary.PrintString` "ItemDansMain")
    (`self.MettreObjetDansLaMain` (select `bool` (`KismetMathLibrary.EqualExactly_Vector2DVector2D` (`self.TemporaryCoordinates`) (-11.0 -10.0)) :`true` true) (`self.TemporaryHumanRef`))
    (elif (== (`GameplayStatics.GetPlayerPawn` 0) (`self.TemporaryHumanRef`))
      (cast `/Game/JustATestAssets/Environnement/Usable/Items/Weapon/Ammo/AmmoBP` self
        (:`then`
          (`/Game/JustATestAssets/HUD/Player/HealthManaBar.UpdateLeftWeapon` _healthmanaindicator false)
          (`/Game/JustATestAssets/HUD/Player/HealthManaBar.UpdateRightWeapon` _healthmanaindicator false))
        (:`CastFailed`
          _))
      (`self.DestroyActorEvent`))))

(event `MettreObjetDansLaMain`
  (params (Gauche :type Boolean) (HumanRef :type "/Game/JustATestAssets/Environnement/Pawns/Humans/ControlableCharacter Object Reference"))
  (bind _staticmeshcomponent (`self.StaticMeshComponent`))
  (bind _staticmeshcomponent_2 (`self.StaticMeshComponent`))
  (bind _temporaryhumanref (`self.TemporaryHumanRef`))
  (bind _temporaryhumanref_2 (`self.TemporaryHumanRef`))
  (bind (_returnvalue_location _returnvalue_rotation) (`KismetMathLibrary.BreakTransform` (`KismetMathLibrary.SelectTransform` (`self.CorrectionLeft`) (`self.CorrectionRight`) (`self.LeftHandWeapon`))))
  (bind _humananimbpreference (`/Game/JustATestAssets/Environnement/Pawns/Humans/ControlableCharacter.HumanAnimBpReference` _temporaryhumanref))
  (bind _bodyscale_x (`KismetMathLibrary.BreakVector` (`/Game/JustATestAssets/Environnement/Pawns/Humans/ControlableCharacter.BodyScale` _temporaryhumanref)))
  (bind _handleftattachfirstperson (`/Game/JustATestAssets/Environnement/Pawns/Humans/ControlableCharacter.HandLeftAttachFirstPerson` _temporaryhumanref_2))
  (bind _returnvalue (and (`Pawn.IsPlayerControlled` _temporaryhumanref) (`Pawn.IsLocallyControlled` _temporaryhumanref)))
  (bind _healthmanaindicator (`/Game/JustATestAssets/HUD/Player/PlayerHud.HealthManaIndicator` (`/Game/JustATestAssets/Environnement/Pawns/Humans/ControlableCharacter.PlayerHud` _temporaryhumanref)))
  ;[1 1 1] MettreObjetDansMain
  (bind _output_get (set `self.TemporaryHumanRef` HumanRef))
  (`self.StopItem` (`self.StaticMeshComponent`))
  (`self.AdditionalElementToChangeWhenEquip`)
  (if (`self.TwoHands`)
    (set `/Game/JustATestAssets/Environnement/Pawns/Humans/ControlableCharacter.ItemMainGauche` self _output_get)
    (set `/Game/JustATestAssets/Environnement/Pawns/Humans/ControlableCharacter.ItemMainDroite` self _output_get)
    (`SceneComponent.K2_AttachToComponent` _staticmeshcomponent _handleftattachfirstperson "None" "SnapToTarget" "SnapToTarget" "KeepWorld" true)
    (`self.WaitValidity` _humananimbpreference
      (:`Out`
        (set `/Game/JustATestAssets/Environnement/Pawns/Humans/HumanAnimBP.WeaponInLeftArm` true _humananimbpreference)
        (set `/Game/JustATestAssets/Environnement/Pawns/Humans/HumanAnimBP.WeaponInRightArm` true _humananimbpreference)
        (bind _newtransform (`self.Clamp Tranform in Range` (`self.CorrectionLeft`) (`self.CorrectionRight`) (`KismetMathLibrary.MapRangeClamped` _bodyscale_x 0.5 1.2 0.0 1.0)))
        (`SceneComponent.K2_SetRelativeLocationAndRotation` _staticmeshcomponent_2 (.location _newtransform) (.rotation _newtransform) false false)
        (if _returnvalue
          (`/Game/JustATestAssets/HUD/Player/HealthManaBar.UpdateLeftWeapon` _healthmanaindicator false)
          (`/Game/JustATestAssets/HUD/Player/HealthManaBar.UpdateRightWeapon` _healthmanaindicator false))))
    (else
      (bind _output_get_2 (set `self.LeftHandWeapon` Gauche))
      (if _output_get_2
        (set `/Game/JustATestAssets/Environnement/Pawns/Humans/ControlableCharacter.ItemMainGauche` self _output_get)
        (else
          (set `/Game/JustATestAssets/Environnement/Pawns/Humans/ControlableCharacter.ItemMainDroite` self _output_get)))
      (`SceneComponent.K2_AttachToComponent` _staticmeshcomponent (select `bool` (`self.LeftHandWeapon`) :`false` (`/Game/JustATestAssets/Environnement/Pawns/Humans/ControlableCharacter.HandRightAttachFirstPerson` _temporaryhumanref_2) :`true` _handleftattachfirstperson) "None" "SnapToTarget" "SnapToTarget" "KeepWorld" true)
      (`self.WaitValidity` _humananimbpreference
        (:`Out`
          (if (`self.LeftHandWeapon`)
            (set `/Game/JustATestAssets/Environnement/Pawns/Humans/HumanAnimBP.WeaponInLeftArm` true _humananimbpreference)
            (else
              (set `/Game/JustATestAssets/Environnement/Pawns/Humans/HumanAnimBP.WeaponInRightArm` true _humananimbpreference)))
          (`SceneComponent.K2_SetRelativeLocationAndRotation` _staticmeshcomponent_2 _returnvalue_location _returnvalue_rotation false false)
          (if _returnvalue
            (if (`self.LeftHandWeapon`)
              (`/Game/JustATestAssets/HUD/Player/HealthManaBar.UpdateLeftWeapon` _healthmanaindicator false)
              (else
                (`/Game/JustATestAssets/HUD/Player/HealthManaBar.UpdateRightWeapon` _healthmanaindicator false)))))))))

(event `/Game/JustATestAssets/Environnement/Pawns/Humans/InteractionEnvironment.GetItemInformation`
  (params (ItemInfo :type "/Game/JustATestAssets/Environnement/Usable/Items/ItemAimInfo Structure") (HumanRef :type "/Game/JustATestAssets/Environnement/Pawns/Humans/ControlableCharacter Object Reference"))
  ;[1 1 1] ResendInformation
  (message `/Game/JustATestAssets/Environnement/Pawns/Humans/InteractionEnvironment.GetItemInformation` HumanRef (`self.AimInformation`) null))

(event `AdditionalElementToChangeWhenEquip`
  ;[1 1 1] Changement additionnel pour les enfants
)

(event `AdditionalElementToChangeWhenStopEquip`
  ;[1 1 1] Changement additionnel pour les enfants
)

(event `self.ReceiveTick`
  (params (DeltaSeconds :type "Float (single-precision)"))
  (bind _returnvalue (`SceneComponent.GetComponentVelocity` (`self.StaticMeshComponent`)))
  ;[1 1 1] Velocité en temps réel
  (if (> (`KismetMathLibrary.VSize` _returnvalue) (`self.ChocSoundSpeedMin`))
    (set `self.VelocityDirection` _returnvalue)
    (else
      (set `self.VelocityDirection` (0.0 0.0 0.0)))))

(event `UpdateAdditionalInformation`
  ;[1 1 1] Update add info
)

(event `self.ReceiveBeginPlay`
  ;[1 1 1] Component Hit
  (add `PrimitiveComponent.OnComponentHit` (`self.StaticMeshComponent`) (delegate `Choc`)))

(event `UseAdditionalInformation`
  (params (AdditionalInformation :type "Array of Float (double-precision)"))
  ;[1 1 1] Update add info
)

(event `Choc`
  (params (HitComponent :type "PrimitiveComponent Object Reference") (OtherActor :type "Actor Object Reference") (OtherComp :type "PrimitiveComponent Object Reference") (NormalImpulse :type "Vector Structure") (Hit :type "HitResult Structure (by ref)"))
  (bind _velocitydirection (`self.VelocityDirection`))
  ;[1 1 1] Choc
  (if (== (`self.GetOwner`) (`GameplayStatics.GetPlayerPawn` 0))
    (`|ExecutionSequence`
      (:`then_0`
        (`self.ChocLocal` OtherActor _velocitydirection))
      (:`then_1`
        (`self.ChocServer` OtherActor _velocitydirection)))))

(event `ChocLocal`
  (params (ActorTouched :type "Actor Object Reference") (VelocityDirection :type "Vector Structure"))
  (bind _returnvalue (`KismetMathLibrary.VSize` VelocityDirection))
  (bind _itemimpact (`self.ItemImpact`))
  (bind _chocsoundspeedmin (`self.ChocSoundSpeedMin`))
  (bind (_remainder _returnvalue_2) (`KismetMathLibrary.FMod` (- _returnvalue 600.0) 100.0))
  ;[1 1 1] Choc
  (if (> _returnvalue _chocsoundspeedmin)
    (`AudioComponent.SetFloatParameter` _itemimpact "Volume" (`KismetMathLibrary.MapRangeClamped` _returnvalue _chocsoundspeedmin (`self.ChocSoundSpeedMax`) 0.25 1.0))
    (`AudioComponent.Play` _itemimpact 0.0)
    (if (> _returnvalue 600.0)
      (set `self.VelocityAfterHit` VelocityDirection)
      (message `/Game/JustATestAssets/Environnement/Pawns/Humans/InteractionEnvironment.ApplyEffectInterface` ActorTouched _returnvalue_2 (* (`KismetMathLibrary.Normal` VelocityDirection) (* _returnvalue_2 (`self.StrengthFactor`))) "None" true))))

(event `ChocServer`
  (params (ActorTouched :type "Actor Object Reference") (VelocityDirection :type "Vector Structure"))
  ;[1 1 1] Choc
  (`self.ChocMulti` ActorTouched VelocityDirection))

(event `ChocMulti`
  (params (ActorTouched :type "Actor Object Reference") (VelocityDirection :type "Vector Structure"))
  ;[1 1 1] Choc
  (if (not (== (`self.GetOwner`) (`GameplayStatics.GetPlayerPawn` 0)))
    (`self.ChocLocal` ActorTouched VelocityDirection)))

(fn `Clamp Tranform in Range`
  (params (TransformMin :type "Transform Structure") (TransformMax :type "Transform Structure") (Value :type "Float (double-precision)"))
  (returns (NewTransform :type "Transform Structure"))
  (return (`KismetMathLibrary.MakeTransform` (`KismetMathLibrary.MakeVector` (`KismetMathLibrary.MapRangeClamped` Value 0.0 1.0 (.x (.location TransformMin)) (.x (.location TransformMax))) (`KismetMathLibrary.MapRangeClamped` Value 0.0 1.0 (.y (.location TransformMin)) (.y (.location TransformMax))) (`KismetMathLibrary.MapRangeClamped` Value 0.0 1.0 (.z (.location TransformMin)) (.z (.location TransformMax)))) (`KismetMathLibrary.MakeRotator` (`KismetMathLibrary.MapRangeClamped` Value 0.0 1.0 (.roll (.rotation TransformMin)) (.roll (.rotation TransformMax))) (`KismetMathLibrary.MapRangeClamped` Value 0.0 1.0 (.pitch (.rotation TransformMin)) (.pitch (.rotation TransformMax))) (`KismetMathLibrary.MapRangeClamped` Value 0.0 1.0 (.yaw (.rotation TransformMin)) (.yaw (.rotation TransformMax)))))))

(fn `ItemCooldown`
  (returns (ItemCooldown :type Boolean))
  (locals (FuturCooldownResultLocal :type Boolean :default false))
  (bind _temporaryhumanref (`self.TemporaryHumanRef`))
  (bind _returnvalue (not (`KismetSystemLibrary.IsValid` (`/Game/JustATestAssets/Environnement/Pawns/Humans/ControlableCharacter.ItemMainDroite` _temporaryhumanref))))
  (return (not (select `bool` (`self.TwoHands`) :`false` _returnvalue :`true` (and _returnvalue (not (`KismetSystemLibrary.IsValid` (`/Game/JustATestAssets/Environnement/Pawns/Humans/ControlableCharacter.ItemMainGauche` _temporaryhumanref))))))))

(fn `TrouverPlaceEquipement`
  (params (HumanRef :type "/Game/JustATestAssets/Environnement/Pawns/Humans/ControlableCharacter Object Reference"))
  (returns (PlaceFinded :type Boolean) (Coordinates :type "Vector2D Structure"))
  (locals (HumanRefLocal :type "/Game/JustATestAssets/Environnement/Pawns/Humans/ControlableCharacter Object Reference") (InventoryLocal :type "/Game/JustATestAssets/Environnement/Pawns/Humans/Inventory Structure") (Place :type Boolean :default false) (FailWithThisCase :type Boolean) (CoordinatesLocal :type "Vector2D Structure") (CoordinateLooked :type "Vector2D Structure"))
  (bind (_inventorylocal_size _inventorylocal_items) (break `/Game/JustATestAssets/Environnement/Pawns/Humans/Inventory` (`local.InventoryLocal`)))
  (bind (_inventorylocal_size_2 _inventorylocal_items_2) (break `/Game/JustATestAssets/Environnement/Pawns/Humans/Inventory` (`local.InventoryLocal`)))
  (bind (_inventorylocal_size_3 _inventorylocal_items_3) (break `/Game/JustATestAssets/Environnement/Pawns/Humans/Inventory` (`local.InventoryLocal`)))
  (bind (_inventorylocal_size_4 _inventorylocal_items_4) (break `/Game/JustATestAssets/Environnement/Pawns/Humans/Inventory` (`local.InventoryLocal`)))
  (bind _returnvalue (`KismetArrayLibrary.Array_Length` _inventorylocal_items_4))
  (bind _output_get (set `local.HumanRefLocal` HumanRef))
  (set `local.InventoryLocal` (`/Game/JustATestAssets/Environnement/Pawns/Humans/ControlableCharacter.Inventory` _output_get))
  (if (`self.TwoHands`)
    ;[1 1 1] Pour Chaque case avec big item
    (for _index (range 2)
      (set `local.CoordinateLooked` (select `int` _index :`0` (-11.0 -10.0) :`1` (-10.0 -11.0) :!type "Vector2D Structure"))
      (if (`local.FailWithThisCase`)
        (`/Game/JustATestAssets/Environnement/Pawns/Humans/ControlableCharacter.RangerItemMainClient` (`local.HumanRefLocal`) true :!label _label)
        (`/Game/JustATestAssets/Environnement/Pawns/Humans/ControlableCharacter.RangerItemMainClient` (`local.HumanRefLocal`) false :!label _label_2)
        (set `local.Place` true :!label _label_3)
        (set `local.CoordinatesLocal` (-10.0 -11.0))
        (return (`local.Place`) (`local.CoordinatesLocal`))
        (elif (== (`KismetArrayLibrary.Array_Length` _inventorylocal_items_3) 0)
          (set `local.Place` true)
          (set `local.CoordinatesLocal` (`local.CoordinateLooked`))
          (else
            ;[1 1 1] Verifier case de perso avec big item
            (for _array_element _inventorylocal_items_2
              (if (`KismetMathLibrary.EqualExactly_Vector2DVector2D` (`.ItemInventoryPosition_14_F3E2699543AFA2F7C05F2489D68BDBD6` (break `/Game/JustATestAssets/Environnement/Usable/Items/ItemPropertiesInventory` _array_element)) (`local.CoordinateLooked`))
                (set `local.FailWithThisCase` true)
                (break)))))))
    (if (`local.FailWithThisCase`)
      (goto _label)
      (else
        (goto _label_3)))
    (else
      ;[1 1 1] Pour chaque case du perso
      (for _index_2 (range 2)
        (set `local.CoordinateLooked` (select `int` _index_2 :`0` (-11.0 -10.0) :`1` (-10.0 -11.0) :!type "Vector2D Structure"))
        (if (not (`local.Place`))
          (set `local.FailWithThisCase` false)
          (if (== _returnvalue 0)
            (set `local.Place` true)
            (set `local.CoordinatesLocal` (`local.CoordinateLooked`))
            (else
              ;[1 1 1] Verifier case de perso
              (for (_array_element_2 _array_index) _inventorylocal_items
                (if (`local.FailWithThisCase`)
                  _
                  (elif (`KismetMathLibrary.EqualExactly_Vector2DVector2D` (`.ItemInventoryPosition_14_F3E2699543AFA2F7C05F2489D68BDBD6` (break `/Game/JustATestAssets/Environnement/Usable/Items/ItemPropertiesInventory` _array_element_2)) (`local.CoordinateLooked`))
                    (set `local.FailWithThisCase` true)
                    (break)
                    (elif (== _array_index (- _returnvalue 1))
                      (set `local.Place` true)
                      (set `local.CoordinatesLocal` (`local.CoordinateLooked`))))))))))
      (if (`local.Place`)
        _
        (else
          (goto _label_2)))))
  (return (`local.Place`) (`local.CoordinatesLocal`)))

(fn `TrouverPlaceInventaire`
  (params (HumanRef :type "/Game/JustATestAssets/Environnement/Pawns/Humans/ControlableCharacter Object Reference"))
  (returns (PasDePlace :type Boolean) (Colonnes :type Integer) (Lignes :type Integer))
  (locals (HumanRefLocal :type "/Game/JustATestAssets/Environnement/Pawns/Humans/ControlableCharacter Object Reference") (InventoryLocal :type "/Game/JustATestAssets/Environnement/Pawns/Humans/Inventory Structure") (ColoneLocal :type Integer) (LigneLocal :type Integer) (Place :type Boolean :default false) (ColonneObjet :type Integer :default 0) (LigneObjet :type Integer :default 0) (ColoneLocalIndex :type Integer) (LigneLocalIndex :type Integer) (ColonneObjetIndex :type Integer) (LigneObjetIndex :type Integer) (FailWithThisCase :type Boolean))
  (bind (_inventorylocal_size _inventorylocal_items) (break `/Game/JustATestAssets/Environnement/Pawns/Humans/Inventory` (`local.InventoryLocal`)))
  (bind (_inventorylocal_size_2 _inventorylocal_items_2) (break `/Game/JustATestAssets/Environnement/Pawns/Humans/Inventory` (`local.InventoryLocal`)))
  (bind _itemproperties (`self.ItemProperties`))
  (bind _itemproperties_2 (`self.ItemProperties`))
  (bind _itemproperties_3 (`self.ItemProperties`))
  (bind _output_get (set `local.HumanRefLocal` HumanRef))
  ;[1 1 1] Pour chaque case d'inventaire
  (bind _output_get_2 (set `local.InventoryLocal` (`/Game/JustATestAssets/Environnement/Pawns/Humans/ControlableCharacter.Inventory` _output_get)))
  (for _index (range (+ (`KismetMathLibrary.FTrunc` (- (`KismetMathLibrary.BreakVector2D` (break `/Game/JustATestAssets/Environnement/Pawns/Humans/Inventory` _output_get_2)) (`KismetMathLibrary.BreakVector2D` (`.ItemSize_16_1381565F4EECF6FB290DAD9CC98CC2A0` (break `/Game/JustATestAssets/Environnement/Usable/Items/ItemPropertiesInventory` _itemproperties_2))))) 1)) :!label _label
    (if (not (`local.Place`))
      (set `local.ColoneLocal` _index)
      (for _index_2 (range (+ (`KismetMathLibrary.FTrunc` (- (`.Y` (`KismetMathLibrary.BreakVector2D` (break `/Game/JustATestAssets/Environnement/Pawns/Humans/Inventory` _output_get_2))) (`.Y` (`KismetMathLibrary.BreakVector2D` (`.ItemSize_16_1381565F4EECF6FB290DAD9CC98CC2A0` (break `/Game/JustATestAssets/Environnement/Usable/Items/ItemPropertiesInventory` _itemproperties_2)))))) 1))
        (if (not (`local.Place`))
          (set `local.LigneLocal` _index_2)
          ;[1 1 1] Pour chaque case de l'objet à placer
          (for _index_3 (range (+ (`KismetMathLibrary.FTrunc` (- (`KismetMathLibrary.BreakVector2D` (`.ItemSize_16_1381565F4EECF6FB290DAD9CC98CC2A0` (break `/Game/JustATestAssets/Environnement/Usable/Items/ItemPropertiesInventory` _itemproperties))) 1.0)) 1)) :!label _label_2
            (set `local.ColoneLocalIndex` _index_3)
            (for _index_4 (range (+ (`KismetMathLibrary.FTrunc` (- (`.Y` (`KismetMathLibrary.BreakVector2D` (`.ItemSize_16_1381565F4EECF6FB290DAD9CC98CC2A0` (break `/Game/JustATestAssets/Environnement/Usable/Items/ItemPropertiesInventory` _itemproperties)))) 1.0)) 1))
              (set `local.LigneLocalIndex` _index_4)
              (if (== (`KismetArrayLibrary.Array_Length` _inventorylocal_items_2) 0)
                (set `local.Place` true)
                (else
                  ;[1 1 1] Pour chaque autre objet de l'inventaire
                  (for (_array_element _array_index) _inventorylocal_items_2
                    (set `local.ColonneObjet` (`KismetMathLibrary.FTrunc` (`KismetMathLibrary.BreakVector2D` (`.ItemInventoryPosition_14_F3E2699543AFA2F7C05F2489D68BDBD6` (break `/Game/JustATestAssets/Environnement/Usable/Items/ItemPropertiesInventory` _array_element)))))
                    (set `local.LigneObjet` (`KismetMathLibrary.FTrunc` (`.Y` (`KismetMathLibrary.BreakVector2D` (`.ItemInventoryPosition_14_F3E2699543AFA2F7C05F2489D68BDBD6` (break `/Game/JustATestAssets/Environnement/Usable/Items/ItemPropertiesInventory` _array_element))))))
                    (bind _returnvalue (`KismetMathLibrary.FTrunc` (- (`KismetMathLibrary.BreakVector2D` (`.ItemSize_16_1381565F4EECF6FB290DAD9CC98CC2A0` (break `/Game/JustATestAssets/Environnement/Usable/Items/ItemPropertiesInventory` _array_element))) 1.0)))
                    (for _index_5 (range (+ _returnvalue 1))
                      (set `local.ColonneObjetIndex` _index_5)
                      (bind _returnvalue_2 (`KismetMathLibrary.FTrunc` (- (`.Y` (`KismetMathLibrary.BreakVector2D` (`.ItemSize_16_1381565F4EECF6FB290DAD9CC98CC2A0` (break `/Game/JustATestAssets/Environnement/Usable/Items/ItemPropertiesInventory` _array_element)))) 1.0)))
                      (for _index_6 (range (+ _returnvalue_2 1))
                        (set `local.LigneObjetIndex` _index_6)
                        (if (`local.FailWithThisCase`)
                          _
                          (elif (and (== (+ (`local.ColonneObjetIndex`) (`local.ColonneObjet`)) (+ (`local.ColoneLocalIndex`) (`local.ColoneLocal`))) (== (+ (`local.LigneObjetIndex`) (`local.LigneObjet`)) (+ (`local.LigneLocalIndex`) (`local.LigneLocal`))))
                            (set `local.FailWithThisCase` true)
                            (goto _label_2 :!via `Break`)
                            (elif (and (== (`local.ColonneObjetIndex`) _returnvalue) (== (`local.LigneObjetIndex`) _returnvalue_2) (== _array_index (- (`KismetArrayLibrary.Array_Length` _inventorylocal_items) 1)) (== (`KismetMathLibrary.FTrunc` (- (`KismetMathLibrary.BreakVector2D` (`.ItemSize_16_1381565F4EECF6FB290DAD9CC98CC2A0` (break `/Game/JustATestAssets/Environnement/Usable/Items/ItemPropertiesInventory` _itemproperties_3))) 1.0)) (`local.ColoneLocalIndex`)) (== (`KismetMathLibrary.FTrunc` (- (`.Y` (`KismetMathLibrary.BreakVector2D` (`.ItemSize_16_1381565F4EECF6FB290DAD9CC98CC2A0` (break `/Game/JustATestAssets/Environnement/Usable/Items/ItemPropertiesInventory` _itemproperties_3)))) 1.0)) (`local.LigneLocalIndex`)))
                              (set `local.Place` true)
                              (goto _label :!via `Break`)))))))))))
          (set `local.FailWithThisCase` false)))))
  (return (`local.Place`) (`local.ColoneLocal`) (`local.LigneLocal`)))

(fn `UserConstructionScript`
  ;[1 1 1] Sound choc type
  (`AudioComponent.SetIntParameter` (`self.ItemImpact`) "Type" (`self.ItemTypeMaterial`)))