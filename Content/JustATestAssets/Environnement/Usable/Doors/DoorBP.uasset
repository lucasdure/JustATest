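; Usable, lockable door that slides or rotates, with aim information for the player and a red/green status light.
; Use or remote commands drive MoveComponentTo with sounds, scaling duration by current position for mid-move reversals.
; Commands also set lock and light; toggle and close bypass the lock.
; It reports state changes to listed actors and, as a lever, sends command lists on fully opening or closing.
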(event `/Game/JustATestAssets/Environnement/Pawns/Humans/InteractionEnvironment.GetItemInformation`
  (params (ItemInfo :type "/Game/JustATestAssets/Environnement/Usable/Items/ItemAimInfo Structure") (HumanRef :type "/Game/JustATestAssets/Environnement/Pawns/Humans/ControlableCharacter Object Reference"))
  ;[1 1 1] Resend Aim Information
  (if (`self.IsUsable`)
    (message `/Game/JustATestAssets/Environnement/Pawns/Humans/InteractionEnvironment.GetItemInformation` HumanRef (`self.AimInformation`) null)))

(event `self.ReceiveBeginPlay`
  ;[1 1 1] Set loop sound
  (`AudioComponent.SetSound` (`self.Audio`) (`self.OpenCloseLoop`)))

(event `/Game/JustATestAssets/Environnement/Pawns/Humans/InteractionEnvironment.UseObject`
  (params (HumanRef :type "/Game/JustATestAssets/Environnement/Pawns/Humans/ControlableCharacter Object Reference") (Bis :type Boolean) (Instant :type Boolean))
  (bind _rotatingdoor (`self.RotatingDoor`))
  ;[1 1 1] DoorOpenClose
  (if (`self.IsUsable`)
    (if (not (`self.IsLocked`)) :!label _label
      (`|ExecutionSequence` :!label _label_2
        (:`then_0`
          (`AudioComponent.Play` (`self.Audio`) 0.0)
          (`KismetSystemLibrary.MoveComponentTo` (`self.Door`) (select `bool` (or (`self.IsOpen`) (`self.IsOpening`) _rotatingdoor) :`false` (`SceneComponent.RelativeLocation` (`self.DoorPosition`))) (select `bool` (and _rotatingdoor (or (`self.IsClosed`) (`self.IsClosing`))) :`false` (`self.InitRot`) :`true` (`self.AimRotation`)) false false (`self.GetTime`))
          (`AudioComponent.Stop` (`self.Audio`))
          (`GameplayStatics.PlaySoundAtLocation` (`self.OpenCloseOver`) (`SceneComponent.K2_GetComponentLocation` (`self.Door`)) (struct) 1.0 1.0 0.0 "/Game/JustATestAssets/Environnement/Usable/Doors/DoorAttenuation.DoorAttenuation" null null)
          (set `self.IsOpen` (`self.IsOpening`))
          (set `self.IsClosed` (`self.IsClosing`))
          (set `self.IsOpening` false)
          (set `self.IsClosing` false)
          (for _array_element (`self.ActorToSendStateRef`)
            (message `/Game/JustATestAssets/Environnement/Usable/Activator/ActivableInterface.SendStateToActor` _array_element (select `bool` (`self.IsOpen`) :`true` 2)))
          (if (`self.IsLever`)
            (if (`self.IsOpen`)
              (for _array_element_2 (`self.ListOfActorToCommand`)
                (message `/Game/JustATestAssets/Environnement/Usable/Activator/ActivableInterface.SendCommandToActor` (break `/Game/JustATestAssets/Environnement/Usable/Activator/CommandStruture` _array_element_2) (`.CommandId_5_0567DCA54BE6F84D074491A995DBB6FB` (break `/Game/JustATestAssets/Environnement/Usable/Activator/CommandStruture` _array_element_2))))
              (else
                (for _array_element_3 (`self.ListOfActorToUncommand`)
                  (message `/Game/JustATestAssets/Environnement/Usable/Activator/ActivableInterface.SendCommandToActor` (break `/Game/JustATestAssets/Environnement/Usable/Activator/CommandStruture` _array_element_3) (`.CommandId_5_0567DCA54BE6F84D074491A995DBB6FB` (break `/Game/JustATestAssets/Environnement/Usable/Activator/CommandStruture` _array_element_3))))))))
        (:`then_1`
          (set `self.IsOpening` (or (`self.IsClosed`) (`self.IsClosing`)))
          (set `self.IsClosing` (or (`self.IsOpen`) (not (`self.IsOpening`))))
          (`GameplayStatics.PlaySoundAtLocation` (`self.OpenCloseStart`) (`SceneComponent.K2_GetComponentLocation` (`self.Door`)) (struct) 1.0 1.0 0.0 "/Game/JustATestAssets/Environnement/Usable/Doors/DoorAttenuation.DoorAttenuation" null null)
          (set `self.IsOpen` false)
          (set `self.IsClosed` false)
          (for _array_element_4 (`self.ActorToSendStateRef`)
            (message `/Game/JustATestAssets/Environnement/Usable/Activator/ActivableInterface.SendStateToActor` _array_element_4 (select `bool` (`self.IsOpening`) :`false` 1 :`true` 3))))))))

(event `/Game/JustATestAssets/Environnement/Usable/Activator/ActivableInterface.SendCommandToActor`
  (params (CommandId :type Integer))
  ;[1 1 1] DoorOpenClose
  (switch `int` CommandId
    (:`0`
      (goto _label_2))
    (:`1`
      (if (not (or (`self.IsOpening`) (`self.IsOpen`)))
        (goto _label)))
    (:`2`
      (if (not (or (`self.IsClosing`) (`self.IsClosed`)))
        (goto _label_2)))
    (:`3`
      (set `self.IsLocked` false)
      (setmembers `/Game/JustATestAssets/Environnement/Usable/Items/ItemAimInfo` :`StructRef` (`self.AimInformation`) :`Option1` "Ouvrir" :`Option1Usable` true)
      (`self.SetLight`))
    (:`4`
      (set `self.IsLocked` true)
      (setmembers `/Game/JustATestAssets/Environnement/Usable/Items/ItemAimInfo` :`StructRef` (`self.AimInformation`) :`Option1` "Verrouillé" :`Option1Usable` true)
      (`self.SetLight`))
    (:`5`
      (set `self.On` true)
      (`self.SetLight`))
    (:`6`
      (set `self.On` false)
      (`self.SetLight`))))

(fn `GetTime`
  (returns (TimeToClose :type "Float (double-precision)"))
  (bind (_aimrotation_roll _aimrotation_pitch _aimrotation_yaw) (`KismetMathLibrary.BreakRotator` (`self.AimRotation`)))
  (bind (_initrot_roll _initrot_pitch _initrot_yaw) (`KismetMathLibrary.BreakRotator` (`self.InitRot`)))
  (bind _returnvalue (or (`self.IsOpening`) (`self.IsOpen`)))
  (bind (_relativerotation_roll _relativerotation_pitch _relativerotation_yaw) (`KismetMathLibrary.BreakRotator` (`SceneComponent.RelativeRotation` (`self.Door`))))
  (bind _returnvalue_2 (== (- _aimrotation_roll _initrot_roll) 0.0))
  (bind _returnvalue_3 (== (- _aimrotation_pitch _initrot_pitch) 0.0))
  (bind _returnvalue_4 (/ (`KismetMathLibrary.VSize` (`SceneComponent.RelativeLocation` (`self.Door`))) (`KismetMathLibrary.VSize` (`SceneComponent.RelativeLocation` (`self.DoorPosition`)))))
  (bind _returnvalue_5 (`KismetMathLibrary.MapRangeClamped` (select `bool` _returnvalue_2 :`false` _relativerotation_roll :`true` (select `bool` _returnvalue_3 :`false` _relativerotation_pitch :`true` _relativerotation_yaw)) (select `bool` _returnvalue_2 :`false` _aimrotation_roll :`true` (select `bool` _returnvalue_3 :`false` _aimrotation_pitch :`true` _aimrotation_yaw)) (select `bool` _returnvalue_2 :`false` _initrot_roll :`true` (select `bool` _returnvalue_3 :`false` _initrot_pitch :`true` _initrot_yaw)) 1.0))
  (return (* (select `bool` (`self.RotatingDoor`) :`false` (select `bool` _returnvalue :`false` (- 1.0 _returnvalue_4) :`true` _returnvalue_4) :`true` (select `bool` _returnvalue :`false` (- 1.0 _returnvalue_5) :`true` _returnvalue_5)) (`self.TimeMax`))))

(fn `SetLight`
  (`PrimitiveComponent.SetMaterialByName` (`self.Door`) "Light" (select `bool` (`self.On`) :`false` "/Game/JustATestAssets/Environnement/Materials/SimpleMaterials/SimpleColor/Black.Black" :`true` (select `bool` (`self.IsLocked`) :`false` "/Game/JustATestAssets/Environnement/Materials/SimpleMaterials/EmissiveColor/GreenLight.GreenLight" :`true` "/Game/JustATestAssets/Environnement/Materials/SimpleMaterials/EmissiveColor/RedLight.RedLight" :!type "MaterialInterface Object Reference"))))

(fn `UserConstructionScript`
  (bind _islocked (`self.IsLocked`))
  ;[1 1 1] SetLight
  (`PrimitiveComponent.SetMaterialByName` (`self.Door`) "Light" (select `bool` (`self.On`) :`false` "/Game/JustATestAssets/Environnement/Materials/SimpleMaterials/SimpleColor/Black.Black" :`true` (select `bool` (`self.IsLocked`) :`false` "/Game/JustATestAssets/Environnement/Materials/SimpleMaterials/EmissiveColor/GreenLight.GreenLight" :`true` "/Game/JustATestAssets/Environnement/Materials/SimpleMaterials/EmissiveColor/RedLight.RedLight" :!type "MaterialInterface Object Reference")))
  ;[1 1 1] UpdateAimInfo
  (setmembers `/Game/JustATestAssets/Environnement/Usable/Items/ItemAimInfo` :`StructRef` (`self.AimInformation`) :`Option1` (select `bool` _islocked :`false` "Ouvrir" :`true` "Verrouillé" :!type "Text") :`Option1Usable` (select `bool` _islocked :`false` true))
  ;[1 1 1] Rotation initiale
  (set `self.InitRot` (`SceneComponent.RelativeRotation` (`self.Door`)))
  (if (`self.RotatingDoor`)
    ;[1 1 1] SetDoorRotation
    (`SceneComponent.K2_SetRelativeRotation` (`self.Door`) (select `bool` (not (or (`self.IsOpen`) (`self.IsOpening`))) :`false` (`self.AimRotation`) :`true` (`self.InitRot`)) false false)
    (else
      ;[1 1 1] SetDoorLocation
      (`SceneComponent.K2_SetRelativeLocation` (`self.Door`) (select `bool` (not (or (`self.IsOpen`) (`self.IsOpening`))) :`false` (`SceneComponent.RelativeLocation` (`self.DoorPosition`))) false false))))