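; Junction actor between two climbing obstacles that moves the player's ControlableCharacter from one climbing mode to another, such as ledge or pipe.
; BeginPlay pre-traces wall, ground and climb blockage from the End component for the first target mode.
; Tick checks the player's distance to Origin, then CanJoin matches directional input and current climb state.
; SetClimbingMode exits the current climb, then sends wall placement locally and to the server, or grabs the Pipe.
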(event `self.ReceiveBeginPlay`
  (bind _end (`self.End`))
  (bind _returnvalue (`SceneComponent.K2_GetComponentLocation` _end))
  (switch `int` (`self.ClimbingModeAim`)
    (:`0`
      ;[1 1 1] Get WallHit and GroundHit
      (bind _outhit (`KismetSystemLibrary.LineTraceSingle` _returnvalue (+ _returnvalue (* (`SceneComponent.GetForwardVector` _end) 10)) "TraceTypeQuery5" true))
      (bind _output_get (set `self.WallHit` _outhit))
      (bind _returnvalue_2 (+ (`.Location` (`GameplayStatics.BreakHitResult` _output_get)) (`SceneComponent.GetForwardVector` (`self.End`))))
      (bind _returnvalue_3 (+ (0.0 0.0 10.0) _returnvalue_2))
      (bind _outhit_2 (`KismetSystemLibrary.LineTraceSingle` _returnvalue_3 _returnvalue_2 "TraceTypeQuery5" true))
      (set `self.GroundHit` _outhit_2)
      (bind (_outhit_3 _returnvalue_4) (`KismetSystemLibrary.LineTraceSingle` _returnvalue_3 (+ _returnvalue_3 (* (`SceneComponent.GetForwardVector` (`self.End`)) 40)) "TraceTypeQuery5" true))
      (set `self.CantClimb` _returnvalue_4))))

(event `self.ReceiveTick`
  (params (DeltaSeconds :type "Float (single-precision)"))
  (bind _returnvalue (`GameplayStatics.GetPlayerPawn` 0))
  ;[1 1 1] MovePlayer
  (if (< (`KismetMathLibrary.VSize` (- (`self.K2_GetActorLocation` (`GameplayStatics.GetPlayerPawn` 0)) (`SceneComponent.K2_GetComponentLocation` (`self.Origin`)))) (`self.MaxDistance`))
    (if (`self.ActorHasTag` (`GameplayStatics.GetPlayerPawn` 0) "ControlableCharacterTag")
      (`self.ActualCharacterRef`
        (:`then`
          (if (not (== _returnvalue (`self.ActualCharacterRef`)))
            (bind _ascontrolable_character (cast `/Game/JustATestAssets/Environnement/Pawns/Humans/ControlableCharacter` _returnvalue :!label _label))
            (set `self.ActualCharacterRef` _ascontrolable_character)))
        (:`else`
          (goto _label)))
      (bind _canjoin (`self.CanJoin`))
      (if _canjoin
        (`self.SetClimbingMode`)))))

(fn `CanJoin`
  (returns (CanJoin :type Boolean))
  (locals (CharacterRef_Local :type "/Game/JustATestAssets/Environnement/Pawns/Humans/ControlableCharacter Object Reference"))
  (bind _actualcharacterref (`self.ActualCharacterRef`))
  (bind _actualcharacterref_2 (`self.ActualCharacterRef`))
  (bind _avanceraxis (`/Game/JustATestAssets/Environnement/Pawns/Humans/ControlableCharacter.AvancerAxis` _actualcharacterref))
  (bind _gaucheaxis (`/Game/JustATestAssets/Environnement/Pawns/Humans/ControlableCharacter.GaucheAxis` _actualcharacterref))
  (bind _returnvalue (and (`/Game/JustATestAssets/Environnement/Pawns/Humans/ControlableCharacter.InClimbingPosition` _actualcharacterref_2) (not (`/Game/JustATestAssets/Environnement/Pawns/Humans/ControlableCharacter.IsClimbing` _actualcharacterref_2))))
  (return (and (select `int` (`self.DirectionMode`) :`0` (> _avanceraxis 0.0) :`1` (< _avanceraxis 0.0) :`2` (> _gaucheaxis 0.0) :`3` (< _gaucheaxis 0.0)) (select `int` (`self.FromClimb`) :`0` _returnvalue :`1` _returnvalue :`2` (`/Game/JustATestAssets/Environnement/Pawns/Humans/ControlableCharacter.ClimbingPipe` _actualcharacterref_2) :`3` false :`4` false :`5` false :`6` false :`7` false))))

(fn `ChangeClimbingMode`
  (bind _actualcharacterref (`self.ActualCharacterRef`))
  (set `/Game/JustATestAssets/Environnement/Pawns/Humans/HumanAnimBP.IsClimbingPipe` false (`/Game/JustATestAssets/Environnement/Pawns/Humans/ControlableCharacter.HumanAnimBpReference` _actualcharacterref))
  (set `/Game/JustATestAssets/Environnement/Pawns/Humans/ControlableCharacter.ClimbingPipe` false _actualcharacterref)
  (`/Game/JustATestAssets/Environnement/Pawns/Humans/ControlableCharacter.ClimbOver` _actualcharacterref))

(fn `UserConstructionScript`
  (`SphereComponent.SetSphereRadius` (`self.Sphere`) (`self.MaxDistance`) true))