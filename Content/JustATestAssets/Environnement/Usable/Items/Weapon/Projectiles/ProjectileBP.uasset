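; Weapon projectile Blueprint that flies forward, self-destructs after its lifetime, and applies damage and impact effects on hit.
; Each tick it line-traces one frame ahead, ignoring its shooter, then moves by swept offset, destroying itself after consecutive blocked moves.
; Local player shots report hits through WeaponRef, weaponless server shots through OriginalActor, and others just destroy themselves.
; Reported hits spawn a physical-material-based ImpactEffectBP and send damage and impulse to the target.
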(event `self.ReceiveBeginPlay`
  ;[1 1 1] Auto destroy self
  (`KismetSystemLibrary.Delay` (`self.LifeTime`))
  (`self.K2_DestroyActor`))

(event `self.ReceiveTick`
  (params (DeltaSeconds :type "Float (single-precision)"))
  (bind _capsule (`self.Capsule`))
  (bind _hittarget (`self.HitTarget`))
  (bind _capsule_2 (`self.Capsule`))
  (bind _damages (`self.Damages`))
  (bind _returnvalue (`SceneComponent.K2_GetComponentLocation` _capsule_2))
  (bind _returnvalue_2 (* (`SceneComponent.GetForwardVector` (`self.Capsule`)) (`self.ProjectileStrength`)))
  (`|ExecutionSequence`
    (:`then_0`
      ;[1 1 1] Fire on ennemies
      (if (not (`self.Collision`))
        (`/Engine/EditorBlueprintResources/StandardMacros.IsValid` _capsule_2
          (:`Is Valid`
            (bind (_outhit _returnvalue_3) (`KismetSystemLibrary.LineTraceSingle` _returnvalue (+ _returnvalue (* (`SceneComponent.GetForwardVector` _capsule_2) (* (`GameplayStatics.GetWorldDeltaSeconds`) (`self.Speed`)))) "TraceTypeQuery1" true))
            (if _returnvalue_3
              (`/Engine/EditorBlueprintResources/StandardMacros.IsValid` (`self.OriginalActor`)
                (:`Is Valid`
                  (if (not (== (`self.OriginalActor`) (`.HitActor` (`GameplayStatics.BreakHitResult` _outhit))))
                    (set `self.HitTarget` _outhit)
                    (set `self.Collision` true)
                    (if (and (== (`self.OriginalActor`) (`GameplayStatics.GetPlayerPawn` 0)) (not (`self.FromServer`)))
                      (`AudioComponent.Stop` (`self.BulletCue`))
                      (`SceneComponent.SetHiddenInGame` (`self.ParticleSystem`) true false)
                      (`|ExecutionSequence`
                        (:`then_0`
                          (message `/Game/JustATestAssets/Environnement/Usable/Items/Weapon/Projectile_OriginalActor.ProjectileImpact` (`self.WeaponRef`) _hittarget _damages _returnvalue_2))
                        (:`then_1`
                          (`self.GenerateImpactLocal` _hittarget :!label _label)))
                      (elif (not (`KismetSystemLibrary.IsValid` (`self.WeaponRef`)))
                        (if (`KismetSystemLibrary.IsServer`)
                          (`|ExecutionSequence`
                            (:`then_0`
                              (message `/Game/JustATestAssets/Environnement/Usable/Items/Weapon/Projectile_OriginalActor.ProjectileImpact` (`self.OriginalActor`) _hittarget _damages _returnvalue_2))
                            (:`then_1`
                              (goto _label)))
                          (else
                            (`self.K2_DestroyActor` :!label _label_2)))
                        (else
                          (goto _label_2))))))))))))
    (:`then_1`
      ;[1 1 1] Forward speed
      (`/Engine/EditorBlueprintResources/StandardMacros.IsValid` _capsule
        (:`Is Valid`
          (bind _sweephitresult (`SceneComponent.K2_AddLocalOffset` _capsule (`KismetMathLibrary.MakeVector` (* DeltaSeconds (`self.Speed`))) true false))
          (if (`GameplayStatics.BreakHitResult` _sweephitresult)
            (if (`self.SweepCollision`)
              (`self.K2_DestroyActor`)
              (else
                (set `self.SweepCollision` true)))
            (else
              (set `self.SweepCollision` false))))))))

(event `GenerateImpactLocal`
  (params (HitTarget :type "HitResult Structure"))
  ;[1 1 1] Fire on ennemies
  (bind _returnvalue (`|SpawnActorFromClass` "/Game/JustATestAssets/Environnement/Effect/ImpactEffect/ImpactEffectBP.ImpactEffectBP_C" (`KismetMathLibrary.MakeTransform` HitTarget_Location) "AlwaysSpawn" "OverrideRootScale" null null))
  (`/Game/JustATestAssets/Environnement/Effect/ImpactEffect/ImpactEffectBP.GenerateImpact` _returnvalue HitTarget_PhysMat HitTarget_Normal HitTarget_HitComponent HitTarget_HitBoneName)
  (message `/Game/JustATestAssets/Environnement/Pawns/Humans/InteractionEnvironment.ApplyEffectInterface` HitTarget_HitActor (`self.Damages`) (* (`SceneComponent.GetForwardVector` (`self.Capsule`)) (`self.ProjectileStrength`)) HitTarget_HitBoneName false)
  (`self.K2_DestroyActor`))

(fn `UserConstructionScript`
  (`AudioComponent.SetIntParameter` (`self.BulletCue`) "Type" (`self.TypeOfProjectile`)))