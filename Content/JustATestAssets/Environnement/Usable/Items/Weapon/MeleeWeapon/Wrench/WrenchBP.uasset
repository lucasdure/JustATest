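; Wrench melee weapon Blueprint that extends a parent class and adds a WrenchHitParticle component.
; The construction script runs the parent's, then assigns that particle to SceneRef under a WeaponOrientation note.
; TriggerFX branches on Stop but does nothing, as the particle Activate and Deactivate calls are disconnected.
; BeginPlay only calls the parent, and the overlap and Tick events are disabled.
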(event `self.ReceiveBeginPlay`
  (`parent.ReceiveBeginPlay`))

(event `/Game/JustATestAssets/Environnement/Usable/Items/Weapon/WeaponBP.TriggerFX`
  (params (Stop :type Boolean))
  ;[1 1 1] Activer gradient
  (if Stop
    _))

(fn `UserConstructionScript`
  (`parent.UserConstructionScript`)
  (`|ExecutionSequence`
    (:`then_2`
      ;[1 1 1] WeaponOrientation
      (set `self.SceneRef` (`self.WrenchHitParticle`)))))